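; BP_Sarcophagus is an interactable sarcophagus that opens and closes its own inventory screen.
; On BeginPlay it creates a WB_SarcophagusInventory widget, passing in its BPInventoryManager, and keeps it for reuse.
; Interact stores the instigator and toggles the widget, switching player 0 between game-and-UI input with a visible cursor and game-only input without one.
; LookAt returns an empty string.
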(event EventInteract
  (params (Instigator :type Actor%20Object%20Reference))
  (bind _returnvalue (Game|GetPlayerController 0))
  (bind _returnvalue_2 (Game|GetPlayerController 0))
  (bind _sarcohpugus_inventory (Variables|Default|GetSarcohpugus%20Inventory))
  (Variables|Default|SetInteract%20Instigator Instigator)
  (if (Widget|IsVisible (Variables|Default|GetSarcohpugus%20Inventory))
    (Widget|RemovefromParent _sarcohpugus_inventory)
    (Input|SetInputModeGameOnly _returnvalue false)
    (Variables|/Script/Engine.PlayerController|SetbShowMouseCursor _returnvalue_2 false)
    (else
      (UserInterface|Viewport|AddtoViewport _sarcohpugus_inventory 0)
      (Input|SetInputModeGameandUI _returnvalue _sarcohpugus_inventory "DoNotLock" false false)
      (Variables|/Script/Engine.PlayerController|SetbShowMouseCursor _returnvalue_2 true))))

(event EventBeginPlay
  (bind _returnvalue (UserInterface|CreateWidget "/Game/Sarcophagus/Widgets/WB_SarcophagusInventory.WB_SarcophagusInventory_C" 0 (Variables|Default|GetBP_InventoryManager)))
  (Variables|Default|SetSarcohpugus%20Inventory _returnvalue))

(fn ConstructionScript)

(fn Lookat
  (return ""))