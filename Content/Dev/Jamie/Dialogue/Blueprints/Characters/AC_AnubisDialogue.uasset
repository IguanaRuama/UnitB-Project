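; Anubis's dialogue component, scripting the guide of the dead's conversations with the pharaoh's awakened servant.
; Dialogue calls its parent, sets a day-based tree index, then branches into introduction, question menus, or randomized good and poor progress remarks.
; ItemCheck and FoundPersonalCoffin select menus with an extra question, and completed branches set the next index before closing.
; Several milestone reaction lines, such as first curse and quota progress, are unconnected and never run.
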(fn Dialogue
  (|CallParentFunction)
  (CallFunction|SetDialogueTreeIndextoDay)
  (switch int (Variables|Default|GetDialogue%20Tree%20Index)
    (:0
      ;[0.15 0.15 0.15 0.5] Inital Interaction
      (bind _state (CallFunction|AddDialogue "Anubis" "Welcome back to the land of the living, my child. Upon his journey through the underworld, your pharaoh was turned back by Osiris." (Utilities|Array|MakeArray "Continue")))
      (switch Utilities|FlowControl|Switch|SwitchonEnum_Dialogue _state
        (:NewEnumerator0
          (bind _state_2 (CallFunction|AddDialogue "Anubis" "As one of his most loyal, you've been awoken to gather what he needs to make a successful passing." (Utilities|Array|MakeArray "What a great honour.")))
          (switch Utilities|FlowControl|Switch|SwitchonEnum_Dialogue _state_2
            (:NewEnumerator0
              (bind _state_3 (CallFunction|AddDialogue "Anubis" "This place looks adequately equipped for what your highness may need for his journey ahead." (Utilities|Array|MakeArray "Continue")))
              (switch Utilities|FlowControl|Switch|SwitchonEnum_Dialogue _state_3
                (:NewEnumerator0
                  ;[0.15 0.15 0.15 0.5] Inital Dialouge Tree
                  (switch int (CallFunction|ItemCheck) :!label _label
                    (:0
                      (bind (_state_4 _option_index) (CallFunction|AddDialogue "Anubis" "Ask a question of Anubis" (Utilities|Array|MakeArray "Where am I?" "You look familiar" "What do I need to collect")))
                      (LocalVariables|SetOpen%20Index%201 _option_index)
                      (switch Utilities|FlowControl|Switch|SwitchonEnum_Dialogue _state_4
                        (:NewEnumerator0
                          _)))
                    (:1
                      (bind (_state_5 _option_index_2) (CallFunction|AddDialogue "Anubis" "Ask a question of Anubis" (Utilities|Array|MakeArray "Where am I?" "You look familiar" "What do I need to collect" "This digging is hard.")))
                      (LocalVariables|SetOpen%20Index%201 _option_index_2)
                      (switch Utilities|FlowControl|Switch|SwitchonEnum_Dialogue _state_5
                        (:NewEnumerator0
                          _))))
                  (switch int (LocalVariables|GetOpen%20Index%201)
                    (:0
                      (bind _state_6 (CallFunction|AddDialogue "Anubis" "Your home. Yet, a lot of time has passed. Us Gods of old seem all but forgotten. Yet, I must still guide those who are faithful to Anubis and seek to be judged by Osiris." (Utilities|Array|MakeArray "Continue")))
                      (switch Utilities|FlowControl|Switch|SwitchonEnum_Dialogue _state_6
                        (:NewEnumerator0
                          (bind (_state_7 _option_index_3) (CallFunction|AddDialogue "Anubis" "Ask a question of Anubis" (Utilities|Array|MakeArray "Where am I?" "You look familiar" "Why Does he lack these items?")))
                          (switch Utilities|FlowControl|Switch|SwitchonEnum_Dialogue _state_7
                            (:NewEnumerator0
                              (switch int _option_index_3
                                (:0
                                  (bind _state_8 (CallFunction|AddDialogue "Anubis" "Your home. Yet, a lot of time has passed. Us Gods of old seem all but forgotten. Yet, I must still guide those who are faithful to Anubis and seek to be judged by Osiris." (Utilities|Array|MakeArray "Continue")))
                                  (switch Utilities|FlowControl|Switch|SwitchonEnum_Dialogue _state_8
                                    (:NewEnumerator0
                                      (CallFunction|SetDialogueTreeIndex 1)
                                      (CallFunction|CloseConversation))))
                                (:1
                                  (bind _state_9 (CallFunction|AddDialogue "Anubis" "I should. I am known as Anubis, guide of the dead." (Utilities|Array|MakeArray "Continue")))
                                  (switch Utilities|FlowControl|Switch|SwitchonEnum_Dialogue _state_9
                                    (:NewEnumerator0
                                      (CallFunction|SetDialogueTreeIndex 1)
                                      (CallFunction|CloseConversation))))
                                (:2
                                  (bind _state_10 (CallFunction|AddDialogue "Anubis" "You would think someone of such status would be well supplied. At least your wit remains intact beyond the grave. They were stolen hundreds of years ago, by thieves of a different age." (Utilities|Array|MakeArray "Continue")))
                                  (switch Utilities|FlowControl|Switch|SwitchonEnum_Dialogue _state_10
                                    (:NewEnumerator0
                                      (CallFunction|SetDialogueTreeIndex 1)
                                      (CallFunction|CloseConversation))))))))))
                    (:1
                      (bind _state_11 (CallFunction|AddDialogue "Anubis" "I should. I am known as Anubis, guide of the dead." (Utilities|Array|MakeArray "Continue")))
                      (switch Utilities|FlowControl|Switch|SwitchonEnum_Dialogue _state_11
                        (:NewEnumerator0
                          (CallFunction|SetDialogueTreeIndex 1)
                          (CallFunction|CloseConversation))))
                    (:2
                      (bind _state_12 (CallFunction|AddDialogue "Anubis" "The path beyond this world is filled with trials and tribulations.Weapons are key for fighting off beasts, 
Tools to navigate such perilous terrain is also recommended." (Utilities|Array|MakeArray "Continue")))
                      (switch Utilities|FlowControl|Switch|SwitchonEnum_Dialogue _state_12
                        (:NewEnumerator0
                          (CallFunction|SetDialogueTreeIndex 1)
                          (CallFunction|CloseConversation))))
                    (:3
                      (bind _state_13 (CallFunction|AddDialogue "Anubis" "Perhaps you need upgrade your tools. They say a good worker need not the best tools.. yet in my experience, it helps." (Utilities|Array|MakeArray "Continue")))
                      (switch Utilities|FlowControl|Switch|SwitchonEnum_Dialogue _state_13
                        (:NewEnumerator0
                          (CallFunction|SetDialogueTreeIndex 1)
                          (CallFunction|CloseConversation))))))))))))
    (:1
      (goto _label))
    (:2
      ;[0.15 0.15 0.15 0.5] Day 2 Dialogue Tree
      (switch int (CallFunction|FoundPersonalCoffin)
        (:0
          (bind (_state_14 _option_index_4) (CallFunction|AddDialogue "Anubis" "Ask a question of Anubis" (Utilities|Array|MakeArray "Are you here to help?" "Do I need to contribute everything immediately?" "I've noticed a lot of scarab depictions in this tomb." "Who is the one I serve?")))
          (LocalVariables|SetOption%20Index%202 _option_index_4)
          (switch Utilities|FlowControl|Switch|SwitchonEnum_Dialogue _state_14
            (:NewEnumerator0
              _)))
        (:1
          (bind (_state_15 _option_index_5) (CallFunction|AddDialogue "Anubis" "Ask a question of Anubis" (Utilities|Array|MakeArray "Are you here to help?" "Do I need to contribute everything immediately?" "I've noticed a lot of scarab depictions in this tomb." "Who is the one I serve?" "Why is my coffin empty?")))
          (LocalVariables|SetOption%20Index%202 _option_index_5)
          (switch Utilities|FlowControl|Switch|SwitchonEnum_Dialogue _state_15
            (:NewEnumerator0
              _))))
      (switch int (LocalVariables|GetOption%20Index%202)
        (:0
          (bind _state_16 (CallFunction|AddDialogue "Anubis" "I am here simply to guide. As the guide of the dead, it is my sworn duty to help those pass through the afterlife." (Utilities|Array|MakeArray "Continue")))
          (switch Utilities|FlowControl|Switch|SwitchonEnum_Dialogue _state_16
            (:NewEnumerator0
              (CallFunction|SetDialogueTreeIndex 2)
              (CallFunction|CloseConversation))))
        (:1
          (bind (_state_17 _option_index_6) (CallFunction|AddDialogue "Anubis" "Your pharaoh should be appeased by a little progress each day. Yet I would not slack; Your ruler knows how to lay a mean curse should you not appease." (Utilities|Array|MakeArray "What do curses entail?" "What else are items used for?")))
          (switch Utilities|FlowControl|Switch|SwitchonEnum_Dialogue _state_17
            (:NewEnumerator0
              (switch int _option_index_6
                (:0
                  (bind _state_18 (CallFunction|AddDialogue "Anubis" "Who's to say... His powers are not my own. But it would hinder your abilities to do your job." (Utilities|Array|MakeArray "Why hinder me with a curse if he is reliant on my help?")))
                  (switch Utilities|FlowControl|Switch|SwitchonEnum_Dialogue _state_18
                    (:NewEnumerator0
                      (bind _state_19 (CallFunction|AddDialogue "Anubis" "Counterproductive, I will admit. Yet, his highness does tend to let his emotions best him. Such a quarrel is between you and him. I exist just to guide." (Utilities|Array|MakeArray "Continue")))
                      (switch Utilities|FlowControl|Switch|SwitchonEnum_Dialogue _state_19
                        (:NewEnumerator0
                          (CallFunction|SetDialogueTreeIndex 2)
                          (CallFunction|CloseConversation))))))
                (:1
                  (bind _state_20 (CallFunction|AddDialogue "Anubis" "Excess items can be sacrificed for Knowledge of the Dead. Such knowledge can heighten your abilities. Be tactical about what you keep and what you leave." (Utilities|Array|MakeArray "Continue")))
                  (switch Utilities|FlowControl|Switch|SwitchonEnum_Dialogue _state_20
                    (:NewEnumerator0
                      (CallFunction|SetDialogueTreeIndex 2)
                      (CallFunction|CloseConversation))))))))
        (:2
          (bind _state_21 (CallFunction|AddDialogue "Anubis" "Your pharaoh had a fondness for such beetles." (Utilities|Array|MakeArray "The pharaoh liked beetles?")))
          (switch Utilities|FlowControl|Switch|SwitchonEnum_Dialogue _state_21
            (:NewEnumerator0
              (bind _state_22 (CallFunction|AddDialogue "Anubis" "Yes, Scarabs, specifically. During his youth, he would collect and care for them. Under such a tough exterior, a simple soul with an affinity for small creatures." (Utilities|Array|MakeArray "What else can you tell me about the pharoah?")))
              (switch Utilities|FlowControl|Switch|SwitchonEnum_Dialogue _state_22
                (:NewEnumerator0
                  (bind _state_23 (CallFunction|AddDialogue "Anubis" "So much to say.. Can a man be summarised in just words? A young soul at the throne, a boy fond of merdjed and cats. Put anyone in a position such as he at some a young age, and would they be a more just ruler? Difficult to say if some of his cruel deeds could be passed off to the inexperience of his youth, or corruption of his heart. Either way, that will be decided before Osiris." (Utilities|Array|MakeArray "Continue")))
                  (switch Utilities|FlowControl|Switch|SwitchonEnum_Dialogue _state_23
                    (:NewEnumerator0
                      (CallFunction|SetDialogueTreeIndex 2)
                      (CallFunction|CloseConversation))))))))
        (:3
          (bind _state_24 (CallFunction|AddDialogue "Anubis" "I suppose a multitude of millennia hay leave some gaps in mortal memories... The Pharaoh ruler of Egypt. You served faithfully under him until you both perished just days apart." (Utilities|Array|MakeArray "Continue")))
          (switch Utilities|FlowControl|Switch|SwitchonEnum_Dialogue _state_24
            (:NewEnumerator0
              (CallFunction|SetDialogueTreeIndex 2)
              (CallFunction|CloseConversation))))
        (:4
          (bind (_state_25 _option_index_7) (CallFunction|AddDialogue "Anubis" "The ruler considers himself more important. He did not supply you with such things." (Utilities|Array|MakeArray "Is he more important?" "Do I need items in my coffin?" "Did I not leave myself any tools for my journey?")))
          (switch Utilities|FlowControl|Switch|SwitchonEnum_Dialogue _state_25
            (:NewEnumerator0
              (switch int _option_index_7
                (:0
                  (bind _state_26 (CallFunction|AddDialogue "Anubis" "Important...Ask this not of me to decide. All that matters is the judgement of Osiris." (Utilities|Array|MakeArray "Continue")))
                  (switch Utilities|FlowControl|Switch|SwitchonEnum_Dialogue _state_26
                    (:NewEnumerator0
                      (CallFunction|SetDialogueTreeIndex 2)
                      (CallFunction|CloseConversation))))
                (:1
                  (bind _state_27 (CallFunction|AddDialogue "Anubis" "That would depend. Do you plan on passing through to the Duat? Such a journey would be troublesome empty handed." (Utilities|Array|MakeArray "Can I tend to my own needs after assisting the one I serve?")))
                  (switch Utilities|FlowControl|Switch|SwitchonEnum_Dialogue _state_27
                    (:NewEnumerator0
                      (bind _state_28 (CallFunction|AddDialogue "Anubis" "You were an efficient worker in life, for sure. If that work ethic survived beyond your mortal plane, perhaps you have the necessary means to tend to both your own needs and the Pharaoh. For after all, your time in this land is almost at its end." (Utilities|Array|MakeArray "What if I don't have time to serve us both?")))
                      (switch Utilities|FlowControl|Switch|SwitchonEnum_Dialogue _state_28
                        (:NewEnumerator0
                          (bind _state_29 (CallFunction|AddDialogue "Anubis" "Ah. Do not all of us have the free will of choice? Yet if your decisions are unjust, you should fear the scale." (Utilities|Array|MakeArray "Scale?")))
                          (switch Utilities|FlowControl|Switch|SwitchonEnum_Dialogue _state_29
                            (:NewEnumerator0
                              (bind _state_30 (CallFunction|AddDialogue "Anubis" "Beyond just my guidance, I must weigh your heart before Osiris. Make sure your actions on this Earth are just, and you reach greater pastures. Yet, your time on this plane is limited." (Utilities|Array|MakeArray "Will I meet Osiris?")))
                              (switch Utilities|FlowControl|Switch|SwitchonEnum_Dialogue _state_30
                                (:NewEnumerator0
                                  (bind _state_31 (CallFunction|AddDialogue "Anubis" "All who make it through the Duat will be judged before him. If you plan on succeeding your journey, then yes." (Utilities|Array|MakeArray "Continue")))
                                  (switch Utilities|FlowControl|Switch|SwitchonEnum_Dialogue _state_31
                                    (:NewEnumerator0
                                      (CallFunction|SetDialogueTreeIndex 2)
                                      (CallFunction|CloseConversation))))))))))))
                (:2
                  (bind (_state_32 _option_index_8) (CallFunction|AddDialogue "Anubis" "Alas... some are too poor to supply themselves with what is necessary." (Utilities|Array|MakeArray "Why did the pharaoh not supply me with items upon death?" "What IS necessary?")))
                  (switch Utilities|FlowControl|Switch|SwitchonEnum_Dialogue _state_32
                    (:NewEnumerator0
                      (switch int _option_index_8
                        (:0
                          (bind _state_33 (CallFunction|AddDialogue "Anubis" "Not for me to say. Such matters are beneath me." (Utilities|Array|MakeArray "Continue")))
                          (switch Utilities|FlowControl|Switch|SwitchonEnum_Dialogue _state_33
                            (:NewEnumerator0
                              (CallFunction|SetDialogueTreeIndex 2)
                              (CallFunction|CloseConversation))))
                        (:1
                          (bind _state_34 (CallFunction|AddDialogue "Anubis" "The Duat is a treacherous journey. If one wishes to reach Aaru, all sorts of items may aid them on their trip I suggest a few of each." (Utilities|Array|MakeArray "Aaru?")))
                          (switch Utilities|FlowControl|Switch|SwitchonEnum_Dialogue _state_34
                            (:NewEnumerator0
                              (bind _state_35 (CallFunction|AddDialogue "Anubis" "Interesting.. I suppose a few thousand years of slumber does rattle your memory. The field of reeds. Where all those worthy in life end after death." (Utilities|Array|MakeArray "Continue")))
                              (switch Utilities|FlowControl|Switch|SwitchonEnum_Dialogue _state_35
                                (:NewEnumerator0
                                  (CallFunction|SetDialogueTreeIndex 2)
                                  (CallFunction|CloseConversation))))))))))))))))
    (:3
      ;[0.15 0.15 0.15 0.5] Good Progress Responses
      (switch int (Math|Random|RandomIntegerinRange 0 4)
        (:0
          (bind _state_36 (CallFunction|AddDialogue "Anubis" "Your ruler is pleased." (Utilities|Array|MakeArray "Continue")))
          (switch Utilities|FlowControl|Switch|SwitchonEnum_Dialogue _state_36
            (:NewEnumerator0
              (CallFunction|SetDialogueTreeIndex 2)
              (CallFunction|CloseConversation))))
        (:1
          (bind _state_37 (CallFunction|AddDialogue "Anubis" "Your ruler is grateful for your service." (Utilities|Array|MakeArray "Continue")))
          (switch Utilities|FlowControl|Switch|SwitchonEnum_Dialogue _state_37
            (:NewEnumerator0
              (CallFunction|SetDialogueTreeIndex 2)
              (CallFunction|CloseConversation))))
        (:2
          (bind _state_38 (CallFunction|AddDialogue "Anubis" "Seems you're progressing well." (Utilities|Array|MakeArray "Continue")))
          (switch Utilities|FlowControl|Switch|SwitchonEnum_Dialogue _state_38
            (:NewEnumerator0
              (CallFunction|SetDialogueTreeIndex 2)
              (CallFunction|CloseConversation))))
        (:3
          (bind _state_39 (CallFunction|AddDialogue "Anubis" "Loyal in life, loyal beyond life..." (Utilities|Array|MakeArray "Continue")))
          (switch Utilities|FlowControl|Switch|SwitchonEnum_Dialogue _state_39
            (:NewEnumerator0
              (CallFunction|SetDialogueTreeIndex 2)
              (CallFunction|CloseConversation))))
        (:4
          (bind _state_40 (CallFunction|AddDialogue "Anubis" "A faithful servant." (Utilities|Array|MakeArray "Continue")))
          (switch Utilities|FlowControl|Switch|SwitchonEnum_Dialogue _state_40
            (:NewEnumerator0
              (CallFunction|SetDialogueTreeIndex 2)
              (CallFunction|CloseConversation))))))
    (:4
      ;[0.15 0.15 0.15 0.5] Poor Progress Responses
      (switch int (Math|Random|RandomIntegerinRange 0 5)
        (:0
          (bind _state_41 (CallFunction|AddDialogue "Anubis" "Your ruler grows restless." (Utilities|Array|MakeArray "Continue")))
          (switch Utilities|FlowControl|Switch|SwitchonEnum_Dialogue _state_41
            (:NewEnumerator0
              (CallFunction|SetDialogueTreeIndex 2)
              (CallFunction|CloseConversation))))
        (:1
          (bind _state_42 (CallFunction|AddDialogue "Anubis" "He doubts your abilities." (Utilities|Array|MakeArray "Continue")))
          (switch Utilities|FlowControl|Switch|SwitchonEnum_Dialogue _state_42
            (:NewEnumerator0
              (CallFunction|SetDialogueTreeIndex 2)
              (CallFunction|CloseConversation))))
        (:2
          (bind _state_43 (CallFunction|AddDialogue "Anubis" "Failure to appease may incur his wrath..." (Utilities|Array|MakeArray "Continue")))
          (switch Utilities|FlowControl|Switch|SwitchonEnum_Dialogue _state_43
            (:NewEnumerator0
              (CallFunction|SetDialogueTreeIndex 2)
              (CallFunction|CloseConversation))))
        (:3
          (bind _state_44 (CallFunction|AddDialogue "Anubis" "I would move with more haste if you are not to suffer" (Utilities|Array|MakeArray "Continue")))
          (switch Utilities|FlowControl|Switch|SwitchonEnum_Dialogue _state_44
            (:NewEnumerator0
              (CallFunction|SetDialogueTreeIndex 2)
              (CallFunction|CloseConversation))))
        (:4
          (bind _state_45 (CallFunction|AddDialogue "Anubis" "Unfaithful, or inadequate?" (Utilities|Array|MakeArray "Continue")))
          (switch Utilities|FlowControl|Switch|SwitchonEnum_Dialogue _state_45
            (:NewEnumerator0
              (CallFunction|SetDialogueTreeIndex 2)
              (CallFunction|CloseConversation))))
        (:5
          (bind _state_46 (CallFunction|AddDialogue "Anubis" "The one you serve grows restless." (Utilities|Array|MakeArray "Continue")))
          (switch Utilities|FlowControl|Switch|SwitchonEnum_Dialogue _state_46
            (:NewEnumerator0
              (CallFunction|SetDialogueTreeIndex 2)
              (CallFunction|CloseConversation))))))))