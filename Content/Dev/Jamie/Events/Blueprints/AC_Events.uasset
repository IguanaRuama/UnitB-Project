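; Event component that tracks daily Sarcophagus and Personal quotas, advances the day cycle and picks the game's ending.
; BeginPlay shows the events widget; quota updates accumulate into per-day arrays, and EndDay resets totals and energy.
; On the third day, summed quotas select an ending, though only Good and Bad print and the rest are stubs.
; The Heart Scarab ending is unreachable behind the both-fulfilled check, and key 1 prints debug sums.
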(event EventBeginPlay
  (bind _returnvalue (UserInterface|CreateWidget "/Game/Dev/Jamie/Events/Widgets/WB_Events.WB_Events_C"))
  (UserInterface|Viewport|AddtoViewport _returnvalue 0))

(event Input|KeyboardEvents|1
  (params (Key :type Key%20Structure :default "None"))
  (:Pressed
    (CallFunction|DEBUG)))

(fn QuotaCheckUpdateSarcophagus
  (params (Total%20%20Quota :type Float%20%28double-precision%29))
  (bind _output_get (Variables|Default|SetQuota%20Daily%20Total%20Sarcophagus (+ (Variables|Default|GetQuota%20Daily%20Total%20Sarcophagus) (/ Total%20%20Quota 1e+02))))
  (Development|PrintString (Utilities|String|ToString(Float) _output_get))
  (Utilities|Array|SetArrayElem (Variables|Default|GetQuota%20Check%20Sarcophagus) (Variables|Default|GetDaily%20Counter) (Variables|Default|GetQuota%20Daily%20Total%20Sarcophagus) true)
  (return (Variables|Default|GetQuota%20Daily%20Total%20Sarcophagus)))

(fn QuotaCheckUpdatePersonal
  (params (Total%20Quota :type Float%20%28double-precision%29))
  (Variables|Default|SetQuota%20Daily%20Total%20Personal (+ (Variables|Default|GetQuota%20Daily%20Total%20Personal) (/ Total%20Quota 1e+02)))
  (Utilities|Array|SetArrayElem (Variables|Default|GetQuota%20Check%20Personal) (Variables|Default|GetDaily%20Counter) (Variables|Default|GetQuota%20Daily%20Total%20Personal) true)
  (return (Variables|Default|GetQuota%20Daily%20Total%20Personal)))

(fn DEBUG
  (bind (_sarcophagus_sum _personal_sum) (CallFunction|QuotaCheckSum))
  (Development|PrintString (Utilities|String|ToString(Float) _sarcophagus_sum))
  (Development|PrintString (Utilities|String|ToString(Float) _personal_sum)))

(fn EndDay
  (bind _result (Math|Integer|IncrementInt (Variables|Default|GetDaily%20Counter))
    (:%20%20
      (Variables|Default|SetDaily%20Counter _result)
      (Variables|Default|SetQuota%20Daily%20Total%20Sarcophagus 0.0)
      (Variables|Default|SetQuota%20Daily%20Total%20Personal 0.0)
      (Variables|Default|SetDay%20Set? true)
      (Variables|Default|SetEnergy 1.0)
      (if (== (Variables|Default|GetDaily%20Counter) 3)
        (CallFunction|EndingSequenceSelector)))))

(fn QuotaCheckSum
  (LocalVariables|SetLocal%20Sarcophagus%20Sum 0.0)
  (LocalVariables|SetLocal%20Personal%20Sum 0.0)
  (for _array_element (Variables|Default|GetQuota%20Check%20Sarcophagus)
    (LocalVariables|SetLocal%20Sarcophagus%20Sum (+ (LocalVariables|GetLocal%20Sarcophagus%20Sum) _array_element)))
  (for _array_element_2 (Variables|Default|GetQuota%20Check%20Personal)
    (LocalVariables|SetLocal%20Personal%20Sum (+ (LocalVariables|GetLocal%20Personal%20Sum) _array_element_2)))
  (return (LocalVariables|GetLocal%20Sarcophagus%20Sum) (LocalVariables|GetLocal%20Personal%20Sum)))

(fn DaySetCheck
  (Variables|Default|SetDay%20Set? false))

(fn PlayerEndingSequence1
  (Development|PrintString "Good Ending"))

(fn PharaohEndingSequence2
  (Development|PrintString "Bad Ending"))

(fn HaraohandPlayerEndingSequence3)

(fn PharaohandPlayer+HeartScarabBeetleEndingSequence4)

(fn BothUnfulfilledEndingSequence5)

(fn EndingSequence6)

(fn EndingSequence7)

(fn EndingSequenceSelector
  (bind (_sarcophagus_sum _personal_sum) (CallFunction|QuotaCheckSum))
  (LocalVariables|SetSarcophagus%20Sum _sarcophagus_sum)
  (LocalVariables|SetPersonal%20Sum _personal_sum)
  (if (and (>= (LocalVariables|GetPersonal%20Sum) 1.0) (< (LocalVariables|GetSarcophagus%20Sum) 1.0))
    (CallFunction|PlayerEndingSequence1)
    (elif (and (>= (LocalVariables|GetSarcophagus%20Sum) 1.0) (< (LocalVariables|GetPersonal%20Sum) 1.0))
      (CallFunction|PharaohEndingSequence2)
      (elif (and (>= (LocalVariables|GetPersonal%20Sum) 1.0) (>= (LocalVariables|GetSarcophagus%20Sum) 1.0))
        (CallFunction|HaraohandPlayerEndingSequence3)
        (elif (and (Variables|Default|GetScarabBool) (and (>= (LocalVariables|GetPersonal%20Sum) 1.0) (>= (LocalVariables|GetSarcophagus%20Sum) 1.0)))
          (CallFunction|PharaohandPlayer+HeartScarabBeetleEndingSequence4)
          (elif (or (< (LocalVariables|GetPersonal%20Sum) 1.0) (< (LocalVariables|GetSarcophagus%20Sum) 1.0))
            (CallFunction|BothUnfulfilledEndingSequence5)
            (else
              (Development|PrintString "No Valid Ending"))))))))