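; Actor component that detects what the player camera is looking at, as a basis for interaction.
; Every tick it sphere-traces forward from the camera up to TraceRange, ignoring its owner, and caches the hit actor in InteractInstigator, clearing it on a miss.
; When the target changes to a new actor, it requests that actor's look-at message and prints it.
; Its own LookAt function returns an empty string.
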(event EventTick
  (params (DeltaSeconds :type Float%20%28single-precision%29))
  (CallFunction|Raycast))

(fn Raycast
  (bind _returnvalue (Game|GetPlayerCameraManager 0))
  (bind _returnvalue_2 (Transformation|GetActorLocation _returnvalue))
  (bind (_outhit _returnvalue_3) (Collision|SphereTraceByChannel _returnvalue_2 (+ _returnvalue_2 (* (Transformation|GetActorForwardVector _returnvalue) (Variables|Default|GetTrace%20Range))) 15.0 "TraceTypeQuery3" false (Utilities|Array|MakeArray (Components|GetOwner)) "None"))
  (if _returnvalue_3
    (if (!= (.HitActor (Collision|BreakHitResult _outhit)) (Variables|Default|GetInteract%20Instigator))
      (bind _output_get (Variables|Default|SetInteract%20Instigator (.HitActor (Collision|BreakHitResult _outhit))))
      (bind _messasge (Class|BIInterface|Lookat(Message) _output_get))
      (Development|PrintString (Utilities|String|ToString(Text) _messasge)))
    (else
      (Variables|Default|SetInteract%20Instigator 0))))

(fn Lookat
  (return ""))