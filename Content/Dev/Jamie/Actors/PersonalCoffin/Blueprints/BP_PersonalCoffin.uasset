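; BP_PersonalCoffin is an interactable coffin actor that opens a personal coffin inventory screen.
; It creates the WB_PersonalCoffin widget at BeginPlay, passing in the inventory manager.
; Interact toggles the widget, switching player 0's input mode and mouse cursor to match.
; Any end overlap on UIBox closes the widget and restores game-only input, while LookAt returns empty text.
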(event OnComponentEndOverlap(UIBox)
  (params (OverlappedComponent :type Primitive%20Component%20Object%20Reference) (OtherActor :type Actor%20Object%20Reference) (OtherComp :type Primitive%20Component%20Object%20Reference) (OtherBodyIndex :type Integer))
  (bind _returnvalue (Game|GetPlayerController 0))
  (Widget|RemovefromParent (Variables|Default|GetCoffin%20Inventory))
  (Input|SetInputModeGameOnly _returnvalue false)
  (Variables|/Script/Engine.PlayerController|SetbShowMouseCursor _returnvalue false))

(event EventInteract
  (params (Instigator :type Actor%20Object%20Reference))
  (bind _returnvalue (Game|GetPlayerController 0))
  (bind _returnvalue_2 (Game|GetPlayerController 0))
  (bind _coffin_inventory (Variables|Default|GetCoffin%20Inventory))
  (Variables|Default|SetInteract%20Instigator Instigator)
  (if (Widget|IsVisible (Variables|Default|GetCoffin%20Inventory))
    (Widget|RemovefromParent _coffin_inventory)
    (Input|SetInputModeGameOnly _returnvalue false)
    (Variables|/Script/Engine.PlayerController|SetbShowMouseCursor _returnvalue_2 false)
    (else
      (UserInterface|Viewport|AddtoViewport _coffin_inventory 0)
      (Input|SetInputModeGameandUI _returnvalue _coffin_inventory "DoNotLock" false false)
      (Variables|/Script/Engine.PlayerController|SetbShowMouseCursor _returnvalue_2 true))))

(event EventBeginPlay
  (bind _returnvalue (UserInterface|CreateWidget "/Game/Dev/Jamie/Actors/PersonalCoffin/Widgets/WB_PersonalCoffin.WB_PersonalCoffin_C" 0 (Variables|Default|GetBP_InventoryManager)))
  (Variables|Default|SetCoffin%20Inventory _returnvalue))

(fn ConstructionScript)

(fn Lookat
  (return ""))