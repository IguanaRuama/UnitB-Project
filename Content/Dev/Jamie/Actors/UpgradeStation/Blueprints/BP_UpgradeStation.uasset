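; Upgrade station actor that opens and closes an upgrade inventory UI when interacted with.
; Creates the widget on BeginPlay with an inventory manager reference, then Interact toggles it in the viewport, switching input mode and mouse cursor.
; Any end overlap on UIBox removes the widget and restores game-only input.
; LookAt returns an empty string.
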(event OnComponentEndOverlap(UIBox)
  (params (OverlappedComponent :type Primitive%20Component%20Object%20Reference) (OtherActor :type Actor%20Object%20Reference) (OtherComp :type Primitive%20Component%20Object%20Reference) (OtherBodyIndex :type Integer))
  (bind _returnvalue (Game|GetPlayerController 0))
  (Widget|RemovefromParent (Variables|Default|GetUpgrade%20Inventory))
  (Input|SetInputModeGameOnly _returnvalue false)
  (Variables|/Script/Engine.PlayerController|SetbShowMouseCursor _returnvalue false))

(event EventBeginPlay
  (bind _returnvalue (UserInterface|CreateWidget (Variables|Default|GetClass) 0 (Variables|Default|GetBP_InventoryManager)))
  (Variables|Default|SetUpgrade%20Inventory _returnvalue))

(event EventInteract
  (params (Instigator :type Actor%20Object%20Reference))
  (bind _returnvalue (Game|GetPlayerController 0))
  (bind _returnvalue_2 (Game|GetPlayerController 0))
  (bind _upgrade_inventory (Variables|Default|GetUpgrade%20Inventory))
  (Variables|Default|SetInteract%20Instigator Instigator)
  (if (Widget|IsVisible (Variables|Default|GetUpgrade%20Inventory))
    (Widget|RemovefromParent _upgrade_inventory)
    (Input|SetInputModeGameOnly _returnvalue_2 false)
    (Variables|/Script/Engine.PlayerController|SetbShowMouseCursor _returnvalue false)
    (else
      (UserInterface|Viewport|AddtoViewport _upgrade_inventory 0)
      (Input|SetInputModeGameandUI _returnvalue_2 _upgrade_inventory "DoNotLock" false false)
      (Variables|/Script/Engine.PlayerController|SetbShowMouseCursor _returnvalue true))))

(fn ConstructionScript)

(fn Lookat
  (return ""))