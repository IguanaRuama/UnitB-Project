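; BP_TestGiveItem is an interactable test actor that toggles a WB_TestGiveItem widget on screen.
; It creates the widget once on BeginPlay, and each Interact stores the instigator, then adds or removes the widget based on its visibility.
; The toggle also switches player 0 between game-and-UI and game-only input, showing or hiding the mouse cursor.
; Its Look At function returns an empty string.
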(event EventBeginPlay
  (bind _returnvalue (UserInterface|CreateWidget "/Game/Dev/Jamie/Actors/Items/Blueprints/TestGiveItem/WB_TestGiveItem.WB_TestGiveItem_C"))
  (Variables|Default|SetTest%20Item%20Inventory _returnvalue))

(event EventInteract
  (params (Instigator :type Actor%20Object%20Reference))
  (bind _returnvalue (Game|GetPlayerController 0))
  (bind _returnvalue_2 (Game|GetPlayerController 0))
  (bind _test_item_inventory (Variables|Default|GetTest%20Item%20Inventory))
  (Variables|Default|SetInteract%20Instigator Instigator)
  (if (Widget|IsVisible (Variables|Default|GetTest%20Item%20Inventory))
    (Widget|RemovefromParent _test_item_inventory)
    (Input|SetInputModeGameOnly _returnvalue false)
    (Variables|/Script/Engine.PlayerController|SetbShowMouseCursor _returnvalue_2 false)
    (else
      (UserInterface|Viewport|AddtoViewport _test_item_inventory 0)
      (Input|SetInputModeGameandUI _returnvalue _test_item_inventory "DoNotLock" false false)
      (Variables|/Script/Engine.PlayerController|SetbShowMouseCursor _returnvalue_2 true))))

(fn ConstructionScript)

(fn Lookat
  (return ""))