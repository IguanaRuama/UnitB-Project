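; Interactable sarcophagus that opens and closes its own inventory screen for the player.
; BeginPlay creates the sarcophagus inventory widget and hands it the inventory manager reference.
; Interact stores the instigator, then toggles the widget on the viewport, switching player 0's input mode and mouse cursor to match.
; Look At returns an empty string.
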(event EventInteract
  (params (Instigator :type Actor%20Object%20Reference))
  (bind _returnvalue (Game|GetPlayerController 0))
  (bind _returnvalue_2 (Game|GetPlayerController 0))
  (bind _sarcophagus_inventory (Variables|Default|GetSarcophagus%20Inventory))
  (Variables|Default|SetInteract%20Instigator Instigator)
  (if (Widget|IsVisible (Variables|Default|GetSarcophagus%20Inventory))
    (Widget|RemovefromParent _sarcophagus_inventory)
    (Input|SetInputModeGameOnly _returnvalue false)
    (Variables|/Script/Engine.PlayerController|SetbShowMouseCursor _returnvalue_2 false)
    (else
      (UserInterface|Viewport|AddtoViewport _sarcophagus_inventory 0)
      (Input|SetInputModeGameandUI _returnvalue _sarcophagus_inventory "DoNotLock" false false)
      (Variables|/Script/Engine.PlayerController|SetbShowMouseCursor _returnvalue_2 true))))

(event EventBeginPlay
  (bind _returnvalue (UserInterface|CreateWidget "/Game/Dev/Jamie/Sarcophagus/Widgets/WB_SarcophagusInventory.WB_SarcophagusInventory_C" 0 (Variables|Default|GetBP_InventoryManager)))
  (Variables|Default|SetSarcophagus%20Inventory _returnvalue))

(fn ConstructionScript)

(fn Lookat
  (return ""))