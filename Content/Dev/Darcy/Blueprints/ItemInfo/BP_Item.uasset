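; BP_Item is a poolable item actor that carries an item's name, type, rarity, description and meshes.
; The construction script copies these fields from ItemDetails, storing both the dusty and clean mesh variants.
; On BeginPlay the actor returns itself to the pool through its ACPoolable component.
; The node that would apply the dusty mesh to the StaticMesh component is disconnected, so this Blueprint never sets the visible mesh.
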(event EventBeginPlay
  (Default|ReturntoPool (Variables|Default|GetAC_Poolable)))

(event Collision|EventActorBeginOverlap
  (params (OtherActor :type Actor%20Object%20Reference)))

(event EventTick
  (params (DeltaSeconds :type Float%20%28single-precision%29)))

(fn ConstructionScript
  (bind _itemdetails (Variables|Default|GetitemDetails))
  (Variables|Default|SetdustyMesh (Variables|/Game/Dev/Darcy/Blueprints/ItemInfo/DataAssets/DA_ItemBase.DA_ItemBase_C|GetdustyMesh _itemdetails))
  (Variables|Default|Setname (Variables|/Game/Dev/Darcy/Blueprints/ItemInfo/DataAssets/DA_ItemBase.DA_ItemBase_C|GetName _itemdetails))
  (Variables|Default|SetitemMesh (Variables|/Game/Dev/Darcy/Blueprints/ItemInfo/DataAssets/DA_ItemBase.DA_ItemBase_C|GetcleanMesh _itemdetails))
  (Variables|Default|SetitemType (Variables|/Game/Dev/Darcy/Blueprints/ItemInfo/DataAssets/DA_ItemBase.DA_ItemBase_C|Gettype _itemdetails))
  (Variables|Default|Setrarity (Variables|/Game/Dev/Darcy/Blueprints/ItemInfo/DataAssets/DA_ItemBase.DA_ItemBase_C|Getrarity _itemdetails))
  (Variables|Default|Setdesc (Variables|/Game/Dev/Darcy/Blueprints/ItemInfo/DataAssets/DA_ItemBase.DA_ItemBase_C|Getdesc _itemdetails)))