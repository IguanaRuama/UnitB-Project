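; BP_QTERock is a pooled falling rock for a quick-time event in the excavation game.
; When started, it moves between given start and end locations on a timeline with adjustable speed.
; A finished fall returns it to the pool, ends the site manager's QTE timer and decrements attempts.
; Clicking it stops the fall, pools it, restarts the timer, clears the QTE-active flag and deactivates its Niagara effect.
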(event Custom|startFall
  (params (startLoc :type Vector) (endLoc :type Vector) (speedMult :type Float%20%28double-precision%29))
  (Rendering|SetVisibility (Variables|Default|GetSphere) true false)
  (Transformation|SetActorLocation startLoc false true)
  (Components|Timeline|SetPlayRate (Variables|Default|GetfallingRock) speedMult)
  (bind _alpha (Timeline|fallingRock PlayFromStart)
    (:Update
      (Transformation|SetActorLocation (Math|Vector|Lerp(Vector) endLoc startLoc _alpha) false true))
    (:Finished
      (Default|ReturntoPool (Variables|Default|GetAC_Poolable))
      (Default|EndQTETimer (Variables|Default|GetsiteManager))
      (Default|DecrementAttempts (Variables|Default|GetsiteManager)))))

(event Custom|RockClicked
  (Audio|Components|Audio|Stop (Variables|Default|GetfallingRock))
  (Default|ReturntoPool (Variables|Default|GetAC_Poolable))
  (Rendering|SetVisibility (Variables|Default|GetSphere) true false)
  (Default|RestartQTETimer (Variables|Default|GetsiteManager))
  (Development|PrintString "Clicked")
  (Variables|/Game/Dev/Darcy/Blueprints/ExcavationGame/BP_SiteManager.BP_SiteManager_C|SetqteActive (Variables|Default|GetsiteManager) false)
  ;[1 0.4063 0.2917 0.5] Elliot
  (Components|Activation|Deactivate (Variables|Default|GetNiagara)))

(event EventBeginPlay
  (Default|ReturntoPool (Variables|Default|GetAC_Poolable))
  (bind _returnvalue (Actor|GetActorOfClass "/Game/Dev/Darcy/Blueprints/ExcavationGame/BP_SiteManager.BP_SiteManager_C"))
  (Variables|Default|SetsiteManager _returnvalue))

(event Collision|EventActorBeginOverlap
  (params (OtherActor :type Actor%20Object%20Reference)))

(event EventTick
  (params (DeltaSeconds :type Float%20%28single-precision%29)))

(fn ConstructionScript)