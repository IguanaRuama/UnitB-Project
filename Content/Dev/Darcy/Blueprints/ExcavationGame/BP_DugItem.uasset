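; BP_DugItem is a pooled actor for an item dug up in the excavation game, shown in a dusty or clean state.
; It returns itself to the pool on BeginPlay, and events then assign its item data and teleport it into position.
; The item data supplies the dusty and clean static meshes.
; MagnifySlide uses a timeline to lerp the item along negative Y by a magnify offset.
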(event Custom|SetClean
  (Components|StaticMesh|SetStaticMesh (Variables|Default|GetitemMesh) (Variables|/Game/Dev/Darcy/Blueprints/ItemInfo/DataAssets/DA_ItemBase.DA_ItemBase_C|GetcleanMesh (Variables|Default|GetitemData))))

(event Custom|MagnifySlide
  (bind _self self)
  (bind _returnvalue (Transformation|GetActorLocation _self))
  (bind (_x _y _z) (Math|Vector|BreakVector _returnvalue))
  (Variables|Default|SetinitLoc _returnvalue)
  (Variables|Default|SetfinalLoc (Math|Vector|MakeVector _x (- _y (Variables|Default|GetmagnifyOffset)) _z))
  (bind _aplha (Timeline|Timeline PlayFromStart)
    (:Update
      (Transformation|SetActorLocation self (Math|Vector|Lerp(Vector) (Variables|Default|GetinitLoc) (Variables|Default|GetfinalLoc) _aplha) false true))))

(event Custom|SetPosition
  (params (Loc :type Transform))
  (Transformation|SetActorTransform Loc false true))

(event Custom|SetDustyMesh
  (Components|StaticMesh|SetStaticMesh (Variables|Default|GetitemMesh) (Variables|/Game/Dev/Darcy/Blueprints/ItemInfo/DataAssets/DA_ItemBase.DA_ItemBase_C|GetdustyMesh (Variables|Default|GetitemData))))

(event Custom|SetItem
  (params (itemData :type DA%20Item%20Base%20Object%20Reference))
  (Variables|Default|SetitemData itemData))

(event EventBeginPlay
  (Default|ReturntoPool (Variables|Default|GetAC_Poolable)))

(event Collision|EventActorBeginOverlap
  (params (OtherActor :type Actor%20Object%20Reference)))

(event EventTick
  (params (DeltaSeconds :type Float%20%28single-precision%29)))

(fn ConstructionScript)