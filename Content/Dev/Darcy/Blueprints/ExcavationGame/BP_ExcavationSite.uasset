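; BP_ExcavationSite is a dig site in the excavation game that the player interacts with to start excavating.
; If the site is undug and energy is not zero, interacting activates its Niagara effect and has BP_SiteManager switch the camera to it.
; It restores its dug flag from save data on BeginPlay and saves it through the GameInstance at day end.
; The construction script clears any SiteItem whose rarity mismatches the site's Difficulty.
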(event Custom|SaveSitesData
  (Class|BPISaveGame|SaveExcavationSites(Message) (Game|GetGameInstance) (Utilities|Struct|MakeS_ExcavationSitesSave (Variables|Default|Getdug))))

(event EventBeginPlay
  (bind _returnvalue (Actor|GetActorOfClass "/Game/Dev/Darcy/Blueprints/ExcavationGame/BP_SiteManager.BP_SiteManager_C"))
  (Variables|Default|SetsiteManagerRef _returnvalue)
  (bind _returnvalue_2 (Actor|GetActorOfClass "/Game/Dev/Darcy/Blueprints/DayCycles/BP_DayManager.BP_DayManager_C"))
  (bind _output_get (Variables|Default|SetdayManagerRef _returnvalue_2))
  (EventDispatchers|BindEventtoOnDayEnd _output_get (delegate Custom|SaveSitesData))
  (bind _saveddata (Class|BPISaveGame|GetGameData(Message) (Game|GetGameInstance)))
  (Utilities|IsValid _saveddata
    (:Is%20Valid
      (CallFunction|UseSaveData (Variables|/Game/Dev/Darcy/Blueprints/SaveGame/BP_SaveGame.BP_SaveGame_C|GetsiteSave _saveddata)))))

(event EventOnInteract
  (if (and (not (== (Variables|/Game/Dev/Darcy/Blueprints/DayCycles/BP_DayManager.BP_DayManager_C|GetcurrentEnergyNum (Variables|Default|GetdayManagerRef)) 0)) (== (Variables|Default|Getdug) false))
    (Components|Activation|Activate (Variables|Default|GetNiagara) false)
    ;[0.15 0.15 0.15 0.5] Interface
    (Default|SwitchCameratoSite (Variables|Default|GetsiteManagerRef) self)))

(fn ConstructionScript
  (if (not (Utilities|Enum|Equal(Enum) (Variables|/Game/Dev/Darcy/Blueprints/ItemInfo/DataAssets/DA_ItemBase.DA_ItemBase_C|Getrarity (Variables|Default|GetsiteItem)) (Variables|/Game/Dev/Darcy/Blueprints/ExcavationGame/Difficulties/DA_DifficultyBase.DA_DifficultyBase_C|GetitemRarity (Variables|Default|Getdifficulty))))
    (Variables|Default|SetsiteItem 0)))

(fn UseSaveData
  (params (savedData :type S%20Excavation%20Sites%20Save%20Structure))
  (Variables|Default|Setdug (.dug savedData)))