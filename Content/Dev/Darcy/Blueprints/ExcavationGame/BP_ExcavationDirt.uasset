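; BP_ExcavationDirt is a pooled, draggable dirt piece in the excavation minigame that highlights with an outline material on hover.
; Movement projects the cursor ray onto a drag plane and clamps travel along one direction from the grab point.
; A successful removal slides it away by timeline, returns it to the pool and updates BP_SiteManager's layers.
; Otherwise, timeline-driven ReturnToStart restores the stored transform, also triggered by QTEReset when flagged.
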(event Custom|SuccessfulRemove
  (params (releaseLoc :type Vector) (directionLine :type Vector))
  (bind _alpha (Timeline|endSlide PlayFromStart)
    (:Update
      (Transformation|SetActorLocation (Math|Vector|Lerp(Vector) releaseLoc (+ releaseLoc (* directionLine (Variables|Default|GetoffscreenOffset))) _alpha) false false))
    (:Finished
      (Default|ReturntoPool (Variables|Default|GetAC_Poolable))
      (Default|UpdateLayers (Variables|Default|GetsiteManagerRef) self))))

(event Custom|setStart
  (params (startTransform :type Transform))
  (Variables|Default|SetstartTransform startTransform))

(event Custom|QTEReset
  (if (Variables|Default|GetqteRestart)
    (CallFunction|ReturntoStart (Transformation|GetActorLocation))
    (Variables|Default|SetqteRestart false)))

(event Custom|ReturnToStart
  (params (releaseLoc :type Vector))
  (bind _starttransform (Variables|Default|GetstartTransform))
  (bind _alpha (Timeline|startReturn PlayFromStart)
    (:Update
      (Transformation|SetActorTransform (Math|Transform|MakeTransform (Math|Vector|Lerp(Vector) releaseLoc (.location _starttransform) _alpha) (.rotation _starttransform) (.scale _starttransform))))))

(event Custom|startHover
  (Rendering|Material|SetOverlayMaterial (Variables|Default|GetCube) "/Game/Dev/Darcy/Blueprints/ExcavationGame/M_DirtOutline.M_DirtOutline" :!class /Script/Engine.MeshComponent))

(event Custom|endHover
  (Rendering|Material|SetOverlayMaterial (Variables|Default|GetCube) 0 :!class /Script/Engine.MeshComponent))

(event EventBeginPlay
  (Default|ReturntoPool (Variables|Default|GetAC_Poolable))
  (bind _returnvalue (Actor|GetActorOfClass "/Game/Dev/Darcy/Blueprints/ExcavationGame/BP_SiteManager.BP_SiteManager_C"))
  (Variables|Default|SetsiteManagerRef _returnvalue))

(event Collision|EventActorBeginOverlap
  (params (OtherActor :type Actor%20Object%20Reference)))

(event EventTick
  (params (DeltaSeconds :type Float%20%28single-precision%29)))

(fn ConstructionScript)

(fn Movement
  (params (worldLoc :type Vector) (worldDir :type Vector) (dragPlaneOrigin :type Vector) (dragPlaneNormal :type Vector) (initGrabLoc :type Vector) (dragDirection :type Vector) (initDirtLoc :type Vector))
  (bind _returnvalue (* worldDir 1e+03))
  (bind _returnvalue_2 (+ worldLoc _returnvalue))
  (bind _intersection (Class|KismetMathLibrary|LinePlaneIntersectionOriginNormal worldLoc _returnvalue_2 dragPlaneOrigin dragPlaneNormal))
  (Variables|Default|SetdragLoc _intersection)
  (bind _output_get (Variables|Default|SetreleaseLoc (+ (* (Math|Float|Clamp(Float) (Math|Vector|DotProduct (- _intersection initGrabLoc) dragDirection) 0.0 5e+02) dragDirection) initDirtLoc)))
  (Transformation|SetActorLocation self _output_get false true)
  (return _output_get))