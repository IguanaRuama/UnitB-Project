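; BP_ExcavationCamera is the camera actor for the excavation game, providing shake and zoom effects through timelines.
; CameraShake plays a non-restarting timeline that drives the actor's yaw by a multiplier.
; ZoomIn lowers the actor along Z from a supplied start location, guarded against retriggering while active.
; ZoomOut reuses that timeline, shortening its length and playing it in reverse from the end.
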(event Custom|CameraShake
  (bind _returnvalue (Transformation|GetActorRotation))
  (if (not (Audio|Components|Audio|IsPlaying (Variables|Default|Getshake)))
    (bind _alpha (Timeline|shake PlayFromStart)
      (:Update
        (Transformation|SetActorRelativeRotation (Math|Rotator|MakeRotator (.roll _returnvalue) (.pitch _returnvalue) (* _alpha (Variables|Default|GetshakeRotationMultiplier))))))))

(event Custom|ZoomIn
  (params (startLoc :type Vector))
  (Variables|Default|SetzoomStart startLoc)
  (if (not (Variables|Default|GetzoomActive))
    (Variables|Default|SetzoomActive true)
    (Components|Timeline|SetTimelineLength (Variables|Default|Getzoom) 5.0)
    (bind _alpha (Timeline|zoom PlayFromStart)
      (:Update
        (Transformation|SetActorLocation (Math|Vector|Lerp(Vector) (Variables|Default|GetzoomStart) (Math|Vector|MakeVector (.x (Variables|Default|GetzoomStart)) (.y (Variables|Default|GetzoomStart)) (- (.z (Variables|Default|GetzoomStart)) (Variables|Default|GetzoomDist))) _alpha) false false))
      (:Finished
        (Variables|Default|SetzoomActive false)))))

(event Custom|ZoomOut
  (bind _zoom (Variables|Default|Getzoom))
  (Audio|Components|Audio|Stop _zoom)
  (Components|Timeline|SetTimelineLength _zoom 0.3)
  (Components|Timeline|ReversefromEnd _zoom))

(event EventBeginPlay)

(event Collision|EventActorBeginOverlap
  (params (OtherActor :type Actor%20Object%20Reference)))

(event EventTick
  (params (DeltaSeconds :type Float%20%28single-precision%29)))

(fn ConstructionScript)