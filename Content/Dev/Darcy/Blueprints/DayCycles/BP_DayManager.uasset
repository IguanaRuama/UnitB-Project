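; BP_DayManager runs the day cycle, tracking the day number and an energy budget shown through a WBP_DayDetails widget.
; Spending energy hides an icon and removes the widget; a day can end only at zero energy.
; The OnDayEnd dispatcher advances the day up to a limit, refills energy and saves through the GameInstance, which also supplies saved data on BeginPlay.
; Blessings and curses raise or lower starting energy.
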(event Custom|DecrementEnergy
  (if (not (== (Variables|Default|GetcurrentEnergyNum) 0))
    (bind _result (Math|Integer|DecrementInt (Variables|Default|GetcurrentEnergyNum))
      (:%20%20
        (bind _output_get (Variables|Default|SetcurrentEnergyNum _result))
        (Default|InvisIMG (Variables|Default|GetdayWidget) (Utilities|Array|Get(acopy) (Variables|/Game/Dev/Darcy/Widgets/WBP_DayDetails.WBP_DayDetails_C|GetimgArray (Variables|Default|GetdayWidget)) (Utilities|Operators|Subtract (Variables|Default|GetstartEnergyNum) _output_get 1)))
        (Widget|RemovefromParent (Variables|Default|GetdayWidget))))))

(event Custom|IncrementDay
  (bind _currentdaynum (Variables|Default|GetcurrentDayNum))
  (if (not (== (Variables|Default|GettotalNumDays) _currentdaynum))
    (bind _result (Math|Integer|IncrementInt _currentdaynum)
      (:%20%20
        (Variables|/Game/Dev/Darcy/Widgets/WBP_DayDetails.WBP_DayDetails_C|SetdayNum (Variables|Default|GetdayWidget) _result)
        (CallFunction|ResetEnergy)))))

(event Custom|AddDayWidget
  (UserInterface|Viewport|AddtoViewport (Variables|Default|GetdayWidget) 0))

(event Custom|AttemptToEndDay
  (if (== (Variables|Default|GetcurrentEnergyNum) 0)
    (Default|CallOnDayEnd)
    (else
      (Development|PrintString "NOT TIRED ENOUGH"))))

(event Custom|SaveManagerData
  (Class|BPISaveGame|SaveDayManager(Message) (Game|GetGameInstance) (Utilities|Struct|MakeS_DayManagerSave (Variables|Default|GetstartEnergyNum) (Variables|Default|GetcurrentDayNum))))

(event EventBeginPlay
  (bind _returnvalue (UserInterface|CreateWidget "/Game/Dev/Darcy/Widgets/WBP_DayDetails.WBP_DayDetails_C" (Game|GetPlayerController 0)))
  (bind _output_get (Variables|Default|SetdayWidget _returnvalue))
  (Variables|/Game/Dev/Darcy/Widgets/WBP_DayDetails.WBP_DayDetails_C|SetdayNum _output_get (Variables|Default|GetcurrentDayNum))
  (UserInterface|Viewport|AddtoViewport _output_get 0)
  (EventDispatchers|BindEventtoOnDayEnd (delegate Custom|IncrementDay))
  (EventDispatchers|BindEventtoOnDayEnd (delegate Custom|SaveManagerData))
  (bind _saveddata (Class|BPISaveGame|GetGameData(Message) (Game|GetGameInstance)))
  (Utilities|IsValid _saveddata
    (:Is%20Valid
      (CallFunction|UseSaveGame (Variables|/Game/Dev/Darcy/Blueprints/SaveGame/BP_SaveGame.BP_SaveGame_C|GetdayManagerSave _saveddata)))
    (:Is%20Not%20Valid
      (CallFunction|SetStartingData (Variables|Default|GetstartEnergyNum) (Variables|Default|GetcurrentDayNum)))))

(event Collision|EventActorBeginOverlap
  (params (OtherActor :type Actor%20Object%20Reference)))

(event EventTick
  (params (DeltaSeconds :type Float%20%28single-precision%29)))

(fn ConstructionScript)

(fn AddBlessing
  (if (!= (Variables|Default|GetmaxEnergyNum) (Variables|Default|GetstartEnergyNum))
    (Math|Integer|IncrementInt (Variables|Default|GetstartEnergyNum))))

(fn AddCurse
  (if (!= 1 (Variables|Default|GetstartEnergyNum))
    (Math|Integer|DecrementInt (Variables|Default|GetstartEnergyNum))
    (else
      (Development|PrintString "Game ova"))))

(fn SaveGame
  (Class|BPISaveGame|SaveDayManager(Message) (Game|GetGameInstance) (Utilities|Struct|MakeS_DayManagerSave (Variables|Default|GetstartEnergyNum) (Variables|Default|GetcurrentDayNum))))

(fn UseSaveGame
  (params (saveData :type S%20Day%20Manager%20Save%20Structure))
  (CallFunction|SetStartingData (.startenergynum saveData) (.daynum saveData)))

(fn ResetEnergy
  (bind _startenergynum (Variables|Default|GetstartEnergyNum))
  (Variables|Default|SetcurrentEnergyNum _startenergynum)
  (Default|VisIMGs (Variables|Default|GetdayWidget) _startenergynum))

(fn SetStartingData
  (params (startEnergyNum :type Integer) (currentDayNum :type Integer))
  (bind _output_get (Variables|Default|SetstartEnergyNum startEnergyNum))
  (Variables|Default|SetcurrentEnergyNum _output_get)
  (bind _output_get_2 (Variables|Default|SetcurrentDayNum currentDayNum))
  (Variables|/Game/Dev/Darcy/Widgets/WBP_DayDetails.WBP_DayDetails_C|SetdayNum (Variables|Default|GetdayWidget) _output_get_2))