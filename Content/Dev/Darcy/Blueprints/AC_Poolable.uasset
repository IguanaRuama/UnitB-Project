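; AC_Poolable is an actor component that lets its owning actor be returned to an object pool instead of being destroyed.
; On BeginPlay it caches the transform of the first TargetPoint tagged "Pool" as the pool location.
; ReturnToPool teleports the owner to that transform and hides its root component without propagating to children.
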(event Custom|ReturnToPool
  (Transformation|SetActorTransform (Components|GetOwner) (Variables|Default|GetpoolTransform) false true)
  (Rendering|SetVisibility (Variables|/Script/Engine.Actor|GetRootComponent (Components|GetOwner)) false false))

(event EventBeginPlay
  (bind _outactors (Actor|GetAllActorsOfClasswithTag "/Script/Engine.TargetPoint" "Pool"))
  (Variables|Default|SetpoolTransform (Transformation|GetActorTransform (Utilities|Array|Get(acopy) _outactors))))