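; AC_TEMPInventory is a temporary inventory component that tracks held items and a currently selected item.
; AddItem and RemoveItem validate the item, update the ItemsHeld collection and print a debug message with its name.
; ClearInv empties the collection, and SetCurrentItem stores a valid item as CurrentItem without checking that it is held.
; BeginPlay and Tick are unused.
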(event EventBeginPlay)

(event EventTick
  (params (DeltaSeconds :type Float%20%28single-precision%29)))

(fn AddItem
  (params (itemToAdd :type BP%20Item%20Object%20Reference))
  (Utilities|IsValid itemToAdd
    (:Is%20Valid
      (Utilities|Array|Add (Variables|Default|GetitemsHeld) itemToAdd)
      (Development|PrintString (Utilities|String|Append (Variables|/Game/Dev/Darcy/Blueprints/ItemInfo/BP_Item.BP_Item_C|Getname itemToAdd) " Added to inv")))))

(fn RemoveItem
  (params (itemToRemove :type BP%20Item%20Object%20Reference))
  (Utilities|IsValid itemToRemove
    (:Is%20Valid
      (Utilities|Array|RemoveItem (Variables|Default|GetitemsHeld) itemToRemove)
      (Development|PrintString (Utilities|String|Append (Variables|/Game/Dev/Darcy/Blueprints/ItemInfo/BP_Item.BP_Item_C|Getname itemToRemove) " Removed from inv")))))

(fn ClearInv
  (Utilities|Array|Clear (Variables|Default|GetitemsHeld)))

(fn SetCurrentItem
  (params (selectedItem :type BP%20Item%20Object%20Reference))
  (Utilities|IsValid selectedItem
    (:Is%20Valid
      (Variables|Default|SetcurrentItem selectedItem))))