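; BP_SiteManager runs the excavation minigame, moving the camera to a dig site and managing directional dirt layers stacked over that site's item.
; On game start it shuffles directions into numbered layers, positioning pooled BP_ExcavationDirt actors at tagged TargetPoints.
; Swipe distance decides whether dirt returns to the pool or start; clearing spawns remaining layers and timeline-moves the camera.
; After the last layer a dusting phase shows a progress bar, though its gauge is unfinished.
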(event Custom|SwitchCameraToSite
  (params (site :type BP%20Excavation%20Site%20Object%20Reference))
  (bind _returnvalue (Game|GetPlayerController 0))
  (bind _output_get (Variables|Default|SetcurrentSite site))
  (Variables|Default|SetcurrentCameraLocation (Math|Vector|MakeVector (.x (.location (Transformation|GetActorTransform _output_get))) (.y (.location (Transformation|GetActorTransform _output_get))) (+ (.z (.location (Transformation|GetActorTransform _output_get))) (Variables|Default|GetcameraOffset))))
  (Transformation|SetActorTransform (Variables|Default|GetcameraRef) (Math|Transform|MakeTransform (Variables|Default|GetcurrentCameraLocation) (Variables|Default|GetcameraRotation) "1.000000,1.000000,1.000000") false true)
  (Game|Player|SetViewTargetwithBlend (Game|GetPlayerController 0) (Variables|Default|GetcameraRef) 1.0 "VTBlend_Linear" 0.0 false)
  (Variables|/Script/Engine.PlayerController|SetbShowMouseCursor _returnvalue true)
  (Utilities|IsValid (Variables|Default|GetdigWidget)
    (:Is%20Valid
      (UserInterface|Viewport|AddtoViewport (Variables|Default|GetdigWidget) 0))
    (:Is%20Not%20Valid
      (bind _returnvalue_2 (UserInterface|CreateWidget "/Game/Dev/Darcy/Widgets/WBP_Dig.WBP_Dig_C" _returnvalue))
      (bind _output_get_2 (Variables|Default|SetdigWidget _returnvalue_2))
      (UserInterface|Viewport|AddtoViewport _output_get_2 0))))

(event Custom|BeginGame
  (CallFunction|SwitchCameratoGame)
  (CallFunction|InitLayers)
  (CallFunction|SetItem))

(event Custom|GaugeDusting
  (params (initMousePos :type Vector%202D%20Structure))
  (bind _returnvalue (Math|Vector2D|Vector2DLength))
  ;[0.15 0.15 0.15 0.5] Finish
  (Development|PrintString (Utilities|String|ToString(Float) _returnvalue))
  (bind _output_get (Variables|Default|SetdustProgress (Math|Float|Clamp(Float) (+ (* _returnvalue (Variables|Default|GetshakeSens)) (Variables|Default|GetdustProgress)))))
  (bind _output_get_2 (Variables|/Game/Dev/Darcy/Widgets/WBP_DustBar.WBP_DustBar_C|Setprogress (Variables|Default|GetdustProgressionWidget) _output_get))
  (Development|PrintString (Utilities|String|ToString(Float) _output_get_2)))

(event Custom|SwitchCameraToGame
  (Transformation|SetActorTransform (Variables|Default|GetcameraRef) (Math|Transform|MakeTransform (Variables|Default|GetgameCameraPos) (Variables|Default|GetcameraRotation) "1.000000,1.000000,1.000000") false true))

(event Custom|SpawnLayer
  (params (dirt :type BP%20Excavation%20Dirt%20Object%20Reference) (layerNum :type Integer) (direction :type E_ExcavationDirections%20Enum :default "NewEnumerator0"))
  (Rendering|SetVisibility (Variables|/Game/Dev/Darcy/Actors/ExcavationGame/BP_ExcavationDirt.BP_ExcavationDirt_C|GetCube dirt) true false)
  (bind _output_get (Variables|/Game/Dev/Darcy/Actors/ExcavationGame/BP_ExcavationDirt.BP_ExcavationDirt_C|Setdirection dirt direction))
  (Default|SetStart dirt (Math|Transform|MakeTransform (Math|Vector|MakeVector (.x (.location (.Value (Utilities|Map|Find (Variables|Default|GetdirectionSpawn) _output_get)))) (.y (.location (.Value (Utilities|Map|Find (Variables|Default|GetdirectionSpawn) _output_get)))) (Math|Conversions|ToFloat(Integer) (* layerNum (Variables|Default|GetlayerDistMultiplier)))) (.rotation (.Value (Utilities|Map|Find (Variables|Default|GetdirectionSpawn) _output_get))) "1.000000,1.000000,1.000000"))
  (Transformation|SetActorTransform dirt (Variables|/Game/Dev/Darcy/Actors/ExcavationGame/BP_ExcavationDirt.BP_ExcavationDirt_C|GetstartTransform dirt))
  (Variables|/Game/Dev/Darcy/Actors/ExcavationGame/BP_ExcavationDirt.BP_ExcavationDirt_C|SetlayerNum dirt layerNum)
  (Utilities|Array|RemoveItem (Variables|Default|GetdirtPool) dirt)
  (Utilities|Array|Add (Variables|Default|GetactiveDirt) dirt)
  (Math|Integer|IncrementInt (Variables|Default|GetspawnedLayerNum)))

(event Custom|InitLayers
  (params (Difficulty :type Integer))
  (bind _dirtpool (Variables|Default|GetdirtPool))
  (bind _directions (Variables|Default|Getdirections))
  (for _index (range 0 4)
    (Utilities|Array|Shuffle _directions)
    (for _array_element _directions
      (Utilities|Map|Add (Variables|Default|GetlayerDetails) (Variables|Default|GetlayerNum) _array_element)
      (Math|Integer|IncrementInt (Variables|Default|GetlayerNum))))
  (bind (_keypin _valuepin) (Utilities|Map|ForEachLoop(Map) (Variables|Default|GetlayerDetails))
    (:then
      (if (not (== (Utilities|Array|Length _dirtpool) 0))
        (CallFunction|SpawnLayer (Utilities|Array|Get(acopy) _dirtpool) _keypin _valuepin)))
    (:CompletedPin
      (Variables|Default|SettotalNumLayers (Utilities|Map|Length (Variables|Default|GetlayerDetails))))))

(event Custom|SetItem
  (bind _gamecamerapos (Variables|Default|GetgameCameraPos))
  (bind _output_get (Variables|Default|SetcurrentSiteItem (Variables|/Game/Dev/Darcy/Actors/ExcavationGame/BP_ExcavationSite.BP_ExcavationSite_C|Getitem (Variables|Default|GetcurrentSite))))
  (Transformation|SetActorTransform _output_get (Math|Transform|MakeTransform (Math|Vector|MakeVector (.x _gamecamerapos) (.y _gamecamerapos) (Math|Conversions|ToFloat(Integer) (* (Variables|Default|GettotalNumLayers) (Variables|Default|GetlayerDistMultiplier)))) (Variables|Default|GetcameraRotation) "1.000000,1.000000,1.000000")))

(event Custom|UpdateLayers
  (params (dirt :type BP%20Excavation%20Dirt%20Object%20Reference))
  (bind _gamecamerapos (Variables|Default|GetgameCameraPos))
  (bind _spawnedlayernum (Variables|Default|GetspawnedLayerNum))
  (Utilities|Array|RemoveItem (Variables|Default|GetactiveDirt) dirt)
  (Utilities|Array|Add (Variables|Default|GetdirtPool) dirt)
  (if (== (Variables|Default|GetspawnedLayerNum) (Variables|Default|GettotalNumLayers))
    (if (== (Variables|Default|GetcurrentLayerNum) (Variables|Default|GettotalNumLayers))
      (CallFunction|StartDustingPhase)
      (else
        (Math|Integer|IncrementInt (Variables|Default|GetcurrentLayerNum) :!label _label
          (:%20%20
            (bind _output_get (Variables|Default|SetcurrentCameraLocation (Math|Vector|MakeVector (.x _gamecamerapos) (.y _gamecamerapos) (+ (.z _gamecamerapos) (* (Variables|Default|GetcurrentLayerNum) (Variables|Default|GetlayerDistMultiplier))))))
            (bind _alpha (Timeline|cameraLayerUpdate PlayFromStart)
              (:Update
                (Transformation|SetActorLocation (Variables|Default|GetcameraRef) (Math|Vector|Lerp(Vector) (.location (Transformation|GetActorTransform (Variables|Default|GetcameraRef))) _output_get _alpha) false false)))))))
    (else
      (CallFunction|SpawnLayer (Utilities|Array|Get(acopy) (Variables|Default|GetdirtPool)) _spawnedlayernum (.Value (Utilities|Map|GetKeyValueByIndex (Variables|Default|GetlayerDetails) _spawnedlayernum)))
      (goto _label))))

(event Custom|StartDustingPhase
  (Variables|Default|SetisDusting true)
  (Utilities|IsValid (Variables|Default|GetdustProgressionWidget)
    (:Is%20Valid
      _)
    (:Is%20Not%20Valid
      (bind _returnvalue (UserInterface|CreateWidget "/Game/Dev/Darcy/Widgets/WBP_DustBar.WBP_DustBar_C" (Game|GetPlayerController 0)))
      (Variables|Default|SetdustProgressionWidget _returnvalue)))
  (UserInterface|Viewport|AddtoViewport (Variables|Default|GetdustProgressionWidget) 0))

(event EventBeginPlay
  (bind _outactors (Actor|GetAllActorsOfClass "/Game/Dev/Darcy/Actors/ExcavationGame/BP_ExcavationSite.BP_ExcavationSite_C"))
  (Variables|Default|SetsiteArray _outactors)
  (bind _returnvalue (Actor|GetActorOfClass "/Game/Dev/Darcy/Actors/ExcavationGame/BP_ExcavationCamera.BP_ExcavationCamera_C"))
  (Variables|Default|SetcameraRef _returnvalue)
  (bind _outactors_2 (Actor|GetAllActorsOfClass "/Game/Dev/Darcy/Actors/ExcavationGame/BP_ExcavationDirt.BP_ExcavationDirt_C"))
  (Variables|Default|SetdirtPool _outactors_2)
  (bind _outactors_3 (Actor|GetAllActorsOfClass "/Script/Engine.TargetPoint"))
  (for _array_element _outactors_3
    (if (.ReturnValue (Utilities|Map|Find (Variables|Default|GettagToEnum) (Utilities|Array|Get(acopy) (Variables|/Script/Engine.Actor|GetTags _array_element))))
      (Utilities|Map|Add (Variables|Default|GetdirectionSpawn) (.Value (Utilities|Map|Find (Variables|Default|GettagToEnum) (Utilities|Array|Get(acopy) (Variables|/Script/Engine.Actor|GetTags _array_element)))) (Transformation|GetActorTransform _array_element))
      (elif (== (Utilities|Array|Get(acopy) (Variables|/Script/Engine.Actor|GetTags _array_element)) "Camera")
        (Variables|Default|SetgameCameraPos (.location (Transformation|GetActorTransform _array_element))))))
  (EventDispatchers|BindEventtoOnGameStart (delegate Custom|BeginGame)))

(fn ConstructionScript)

(fn IsCorrectLayer
  (params (selectedDirt :type BP%20Excavation%20Dirt%20Object%20Reference))
  (bind _currentlayernum (Variables|Default|GetcurrentLayerNum))
  (Development|PrintString (Utilities|String|ToString(Integer) _currentlayernum) true true "(R=0.000000,G=1.000000,B=0.448910,A=1.000000)")
  (return (== (Variables|/Game/Dev/Darcy/Actors/ExcavationGame/BP_ExcavationDirt.BP_ExcavationDirt_C|GetlayerNum selectedDirt) _currentlayernum)))

(fn GaugeDirtMovement
  (params (Initial%20Pos :type Vector) (EndPos :type Vector) (dirt :type BP%20Excavation%20Dirt%20Object%20Reference) (directionLine :type Vector))
  (bind _returnvalue (- Initial%20Pos EndPos))
  (if (>= (Math|Float|Sqrt (+ (Math|Float|Square (.x _returnvalue)) (Math|Float|Square (.y _returnvalue)))) 25.0)
    (Default|ReturntoPool dirt EndPos directionLine)
    (else
      (Default|ReturntoStart dirt EndPos))))