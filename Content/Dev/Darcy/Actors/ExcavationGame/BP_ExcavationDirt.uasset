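; Pooled dirt piece for the excavation game that is dragged aside to remove it.
; Movement intersects the cursor ray with a drag plane, then constrains the piece to a clamped, one-way slide along the drag direction.
; Timelines either slide a removed piece onward, hide it and notify BP_SiteManager to update layers, or return it to its start, including on QTE restart.
; It parks at a "Pool"-tagged TargetPoint for reuse.
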(event Custom|SuccessfulRemove
  (params (releaseLoc :type Vector) (directionLine :type Vector))
  (bind _alpha (Timeline|endSlide PlayFromStart)
    (:Update
      (Transformation|SetActorLocation (Math|Vector|Lerp(Vector) releaseLoc (+ releaseLoc (* directionLine (Variables|Default|GetoffscreenOffset))) _alpha) false false))
    (:Finished
      (Rendering|SetVisibility (Variables|Default|GetCube) false false)
      (Default|UpdateLayers (Variables|Default|GetsiteManagerRef) self))))

(event Custom|setStart
  (params (startTransform :type Transform))
  (Variables|Default|SetstartTransform startTransform))

(event Custom|ReturnToPool
  (Transformation|SetActorLocation (.location (Variables|Default|GetpoolTransform)) false true)
  (Rendering|SetVisibility (Variables|Default|GetCube) true false))

(event Custom|QTEReset
  (params (finalLoc :type Vector))
  (if (Variables|Default|GetqteRestart)
    (CallFunction|ReturntoStart finalLoc)
    (Variables|Default|SetqteRestart false)))

(event Custom|ReturnToStart
  (params (releaseLoc :type Vector))
  (bind _starttransform (Variables|Default|GetstartTransform))
  (bind _alpha (Timeline|startReturn PlayFromStart)
    (:Update
      (Transformation|SetActorTransform (Math|Transform|MakeTransform (Math|Vector|Lerp(Vector) releaseLoc (.location _starttransform) _alpha) (.rotation _starttransform) (.scale _starttransform))))))

(event EventBeginPlay
  (bind _outactors (Actor|GetAllActorsOfClasswithTag "/Script/Engine.TargetPoint" "Pool"))
  (bind _output_get (Variables|Default|SetpoolTransform (Transformation|GetActorTransform (Utilities|Array|Get(acopy) _outactors))))
  (Transformation|SetActorTransform _output_get false true)
  (bind _returnvalue (Actor|GetActorOfClass "/Game/Dev/Darcy/Actors/ExcavationGame/BP_SiteManager.BP_SiteManager_C"))
  (Variables|Default|SetsiteManagerRef _returnvalue))

(event Collision|EventActorBeginOverlap
  (params (OtherActor :type Actor%20Object%20Reference)))

(event EventTick
  (params (DeltaSeconds :type Float%20%28single-precision%29)))

(fn ConstructionScript)

(fn Movement
  (params (worldLoc :type Vector) (worldDir :type Vector) (dragPlaneOrigin :type Vector) (dragPlaneNormal :type Vector) (initGrabLoc :type Vector) (dragDirection :type Vector) (initDirtLoc :type Vector))
  (bind _returnvalue (* worldDir 1e+03))
  (bind _returnvalue_2 (+ worldLoc _returnvalue))
  (bind _intersection (Class|KismetMathLibrary|LinePlaneIntersectionOriginNormal worldLoc _returnvalue_2 dragPlaneOrigin dragPlaneNormal))
  (Variables|Default|SetdragLoc _intersection)
  (bind _output_get (Variables|Default|SetreleaseLoc (+ (* (Math|Float|Clamp(Float) (Math|Vector|DotProduct (- _intersection initGrabLoc) dragDirection) 0.0 5e+02) dragDirection) initDirtLoc)))
  (Transformation|SetActorLocation self _output_get false true)
  (return _output_get))