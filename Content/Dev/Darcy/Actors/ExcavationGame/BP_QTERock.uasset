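; BP_QTERock is a pooled falling rock for quick-time events in the excavation game.
; It parks at a "Pool"-tagged TargetPoint, and startFall animates it between supplied start and end locations with a timeline.
; RockClicked stops the fall, returns it to the pool, restarts BP_SiteManager's QTE timer and clears QteActive.
; A completed fall also re-pools it, but ends the manager's timer and decrements attempts.
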(event Custom|startFall
  (params (startLoc :type Vector) (endLoc :type Vector))
  (Rendering|SetVisibility (Variables|Default|GetSphere) true false)
  (Transformation|SetActorLocation startLoc false true)
  (bind _alpha (Timeline|fallingRock PlayFromStart)
    (:Update
      (Transformation|SetActorLocation (Math|Vector|Lerp(Vector) endLoc startLoc _alpha) false true))
    (:Finished
      (Transformation|SetActorLocation (Variables|Default|GetpoolLoc) false true)
      (Default|EndQTETimer (Variables|Default|GetsiteManager))
      (Default|DecrementAttempts (Variables|Default|GetsiteManager)))))

(event Custom|RockClicked
  (Audio|Components|Audio|Stop (Variables|Default|GetfallingRock))
  (Transformation|SetActorLocation (Variables|Default|GetpoolLoc) false false)
  (Rendering|SetVisibility (Variables|Default|GetSphere) true false)
  (Default|RestartQTETimer (Variables|Default|GetsiteManager))
  (Development|PrintString "Clicked")
  (Variables|/Game/Dev/Darcy/Actors/ExcavationGame/BP_SiteManager.BP_SiteManager_C|SetqteActive (Variables|Default|GetsiteManager) false))

(event EventBeginPlay
  (bind _outactors (Actor|GetAllActorsOfClasswithTag "/Script/Engine.TargetPoint" "Pool"))
  (bind _output_get (Variables|Default|SetpoolLoc (Transformation|GetActorLocation (Utilities|Array|Get(acopy) _outactors))))
  (Transformation|SetActorLocation _output_get false false)
  (bind _returnvalue (Actor|GetActorOfClass "/Game/Dev/Darcy/Actors/ExcavationGame/BP_SiteManager.BP_SiteManager_C"))
  (Variables|Default|SetsiteManager _returnvalue))

(event Collision|EventActorBeginOverlap
  (params (OtherActor :type Actor%20Object%20Reference)))

(event EventTick
  (params (DeltaSeconds :type Float%20%28single-precision%29)))

(fn ConstructionScript)