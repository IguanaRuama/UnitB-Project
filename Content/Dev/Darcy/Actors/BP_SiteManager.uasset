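; BP_SiteManager is an actor that manages excavation sites and moves the excavation camera to view a chosen site.
; On BeginPlay it caches all BP_ExcavationSite actors and the BP_ExcavationCamera.
; SwitchCameraToSite teleports that camera above the given site using a height offset and set rotation, then blends player 0's view to it and shows the mouse cursor.
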(event Custom|SwitchCameraToSite
  (params (site :type BP%20Excavation%20Site%20Object%20Reference))
  (bind _returnvalue (Transformation|GetActorTransform site))
  (Variables|Default|SetcameraLocation (Math|Vector|MakeVector (.x (.location _returnvalue)) (.y (.location _returnvalue)) (+ (.z (.location _returnvalue)) (Variables|Default|GetcameraOffset))))
  (Transformation|SetActorTransform (Variables|Default|GetcameraRef) (Math|Transform|MakeTransform (Variables|Default|GetcameraLocation) (Variables|Default|GetcameraRotation) "1.000000,1.000000,1.000000") false true)
  (Game|Player|SetViewTargetwithBlend (Game|GetPlayerController 0) (Variables|Default|GetcameraRef) 1.0 "VTBlend_Linear" 0.0 false)
  (Variables|/Script/Engine.PlayerController|SetbShowMouseCursor (Game|GetPlayerController 0) true))

(event EventBeginPlay
  (bind _outactors (Actor|GetAllActorsOfClass "/Game/Dev/Darcy/Actors/BP_ExcavationSite.BP_ExcavationSite_C"))
  (Variables|Default|SetsiteArray _outactors)
  (bind _returnvalue (Actor|GetActorOfClass "/Game/Dev/Darcy/Actors/BP_ExcavationCamera.BP_ExcavationCamera_C"))
  (Variables|Default|SetcameraRef _returnvalue))

(event Collision|EventActorBeginOverlap
  (params (OtherActor :type Actor%20Object%20Reference)))

(event EventTick
  (params (DeltaSeconds :type Float%20%28single-precision%29)))

(fn ConstructionScript)