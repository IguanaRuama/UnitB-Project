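; BP_Tomb is an interactable tomb actor in the day-cycle system that opens the end-of-day UI.
; OnInteract creates WBP_EndDay on first use, reuses it afterwards, and adds it to the viewport.
; It then switches to UI-only input with a visible cursor, ignores look input and deactivates the player's CharacterMovement.
; BeginPlay caches a BP_ExcavationCamera reference, which the event graph does not otherwise use.
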(event EventBeginPlay
  (bind _returnvalue (Actor|GetActorOfClass "/Game/Dev/Darcy/Actors/BP_ExcavationCamera.BP_ExcavationCamera_C"))
  (Variables|Default|SetcameraRef _returnvalue))

(event Collision|EventActorBeginOverlap
  (params (OtherActor :type Actor%20Object%20Reference)))

(event EventTick
  (params (DeltaSeconds :type Float%20%28single-precision%29)))

(event EventOnInteract
  (bind _returnvalue (Game|GetPlayerController 0))
  (Utilities|IsValid (Variables|Default|GetEndDayWidget)
    (:Is%20Valid
      _)
    (:Is%20Not%20Valid
      (bind _returnvalue_2 (UserInterface|CreateWidget "/Game/Dev/Darcy/Widgets/WBP_EndDay.WBP_EndDay_C" (Game|GetPlayerController 0)))
      (Variables|Default|SetEndDayWidget _returnvalue_2)))
  (UserInterface|Viewport|AddtoViewport (Variables|Default|GetEndDayWidget) 0)
  (Input|SetInputModeUIOnly _returnvalue (Variables|Default|GetEndDayWidget) "DoNotLock" false)
  (Development|PrintString "UI ONLY")
  (Variables|/Script/Engine.PlayerController|SetbShowMouseCursor _returnvalue true)
  (Input|SetIgnoreLookInput _returnvalue true)
  (Components|Activation|Deactivate (Variables|/Script/Engine.Character|GetCharacterMovement (Game|GetPlayerCharacter 0))))

(fn ConstructionScript)