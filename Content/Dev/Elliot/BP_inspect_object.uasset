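; Inspectable world object that shows a prompt widget on overlap and opens an inspect mode where the player rotates, pans and zooms a copy of its mesh.
; Construction copies InteractableMesh to InspectableMesh, raised out of the way with a SceneCaptureComponent2D that renders only that copy.
; Entering and exiting toggle the copy, UI_inspect, cursor and input mapping through BP_FirstPersonPlayerController; exit also resets transform and FOV.
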(event OnComponentBeginOverlap(Sphere)
  (params (OverlappedComponent :type Primitive%20Component%20Object%20Reference) (OtherActor :type Actor%20Object%20Reference) (OtherComp :type Primitive%20Component%20Object%20Reference) (OtherBodyIndex :type Integer) (bFromSweep :type Boolean) (SweepResult :type Hit%20Result%20Structure%20%28by%20ref%29))
  (Rendering|SetVisibility (Variables|Default|GetWidget) true false))

(event OnComponentEndOverlap(Sphere)
  (params (OverlappedComponent :type Primitive%20Component%20Object%20Reference) (OtherActor :type Actor%20Object%20Reference) (OtherComp :type Primitive%20Component%20Object%20Reference) (OtherBodyIndex :type Integer))
  (Rendering|SetVisibility (Variables|Default|GetWidget) false false))

(event Custom|updateZoom
  (params (axis :type Float%20%28double-precision%29))
  (Variables|/Script/Engine.SceneCaptureComponent2D|SetFOVAngle (Variables|Default|GetSceneCaptureComponent2D) (+ (Variables|/Script/Engine.SceneCaptureComponent2D|GetFOVAngle (Variables|Default|GetSceneCaptureComponent2D)) (* axis 3.0))))

(event Custom|update%20mesh%20rotation
  (params (vector%202d :type Vector%202D%20Structure))
  (bind (_x _y) (Math|Vector2D|BreakVector2D vector%202d))
  (bind _inspectable_mesh (Variables|Default|Getinspectable%20mesh))
  (Transformation|SetRelativeRotation _inspectable_mesh (Math|Rotator|CombineRotators (Variables|/Script/Engine.SceneComponent|GetRelativeRotation _inspectable_mesh) (Math|Rotator|MakeRotator 0.0 (* _y -5.0) (* _x -5.0))) false false))

(event Custom|update%20mesh%20location
  (params (vector%202d :type Vector%202D%20Structure))
  (bind (_x _y) (Math|Vector2D|BreakVector2D vector%202d))
  (bind _inspectable_mesh (Variables|Default|Getinspectable%20mesh))
  (bind _default_position (Variables|Default|Getdefault%20position))
  (bind _location (Math|Transform|BreakTransform _default_position))
  (bind (_x_2 _y_2 _z) (Math|Vector|BreakVector _location))
  (Transformation|SetRelativeLocation _inspectable_mesh (Math|Vector|MakeVector 0.0 (Math|Float|Clamp(Float) (+ (.y (Variables|/Script/Engine.SceneComponent|GetRelativeLocation _inspectable_mesh)) (* _x 2.0)) (- _x_2 1e+02) (+ _x_2 1e+02)) (Math|Float|Clamp(Float) (+ (.z (Variables|/Script/Engine.SceneComponent|GetRelativeLocation (Variables|Default|Getinspectable%20mesh))) (* _y 2.0)) (- _z 1e+02) (+ _z 1e+02))) false false))

(event Custom|exit%20inspect%20mode
  (bind _returnvalue (Game|GetPlayerController 0))
  (Development|SetHiddeninGame (Variables|Default|Getinspectable%20mesh) true false)
  (CallFunction|ResetObject)
  (Widget|RemovefromParent (Variables|Default|GetUI%20inspect))
  (Variables|/Script/Engine.PlayerController|SetbShowMouseCursor _returnvalue false)
  (Input|SetInputModeGameOnly _returnvalue false)
  (bind _asbp_first_person_player_controller (Utilities|Casting|CastToBP_FirstPersonPlayerController (Game|GetPlayerController 0)))
  (Default|UpdateInputMapContext _asbp_first_person_player_controller "/Game/Input/IMC_Default.IMC_Default")
  (Variables|/Game/FirstPerson/Blueprints/BP_FirstPersonPlayerController.BP_FirstPersonPlayerController_C|Setinspectable%20Bp _asbp_first_person_player_controller self))

(event Custom|reset%20object
  (Transformation|SetRelativeTransform (Variables|Default|Getinspectable%20mesh) (Variables|Default|Getdefault%20position) false false)
  (Variables|/Script/Engine.SceneCaptureComponent2D|SetFOVAngle (Variables|Default|GetSceneCaptureComponent2D) 9e+01)
  (Class|SceneCaptureComponent|SetCaptureSortPriority (Variables|Default|GetSceneCaptureComponent2D) 1))

(event EventInspectInteract
  (bind _returnvalue (Game|GetPlayerController 0))
  (Development|PrintString "inspect")
  (Class|SceneCaptureComponent|SetCaptureSortPriority (Variables|Default|GetSceneCaptureComponent2D))
  (Development|SetHiddeninGame (Variables|Default|Getinspectable%20mesh) false false)
  (bind _returnvalue_2 (UserInterface|CreateWidget "/Game/Dev/Elliot/UI_inspect.UI_inspect_C"))
  (bind _output_get (Variables|Default|SetUI%20inspect _returnvalue_2))
  (UserInterface|Viewport|AddtoViewport _output_get 0)
  (Variables|/Script/Engine.PlayerController|SetbShowMouseCursor _returnvalue true)
  (Input|SetInputModeGameandUI _returnvalue 0 "DoNotLock" true false)
  (bind _asbp_first_person_player_controller (Utilities|Casting|CastToBP_FirstPersonPlayerController (Game|GetPlayerController 0)))
  (Default|UpdateInputMapContext _asbp_first_person_player_controller "/Game/Dev/Elliot/inspect/IMC_inspect.IMC_inspect")
  (Variables|/Game/FirstPerson/Blueprints/BP_FirstPersonPlayerController.BP_FirstPersonPlayerController_C|Setinspectable%20Bp _asbp_first_person_player_controller self))

(fn ConstructionScript
  (bind _inspectable_mesh (Variables|Default|Getinspectable%20mesh))
  (bind _interactable_mesh (Variables|Default|Getinteractable%20mesh))
  (bind _inspectable_mesh_2 (Variables|Default|Getinspectable%20mesh))
  (bind _scenecapturecomponent2d (Variables|Default|GetSceneCaptureComponent2D))
  (bind _relativelocation (Variables|/Script/Engine.SceneComponent|GetRelativeLocation _scenecapturecomponent2d))
  (bind _relativelocation_2 (Variables|/Script/Engine.SceneComponent|GetRelativeLocation _inspectable_mesh_2))
  (Rendering|SceneCapture|ShowOnlyComponent (Variables|Default|GetSceneCaptureComponent2D) (Variables|Default|Getinspectable%20mesh))
  (Components|StaticMesh|SetStaticMesh _inspectable_mesh (Variables|/Script/Engine.StaticMeshComponent|GetStaticMesh _interactable_mesh))
  (Transformation|SetRelativeTransform _inspectable_mesh (Transformation|GetRelativeTransform _interactable_mesh) false false)
  (Transformation|SetRelativeLocation _inspectable_mesh_2 (Math|Vector|MakeVector (.x _relativelocation_2) (.y _relativelocation_2) 1e+03) false false)
  (Transformation|SetRelativeLocation _scenecapturecomponent2d (Math|Vector|MakeVector (.x _relativelocation) (.y _relativelocation) 1e+03) false false)
  (Variables|Default|Setdefault%20position (Transformation|GetRelativeTransform (Variables|Default|Getinspectable%20mesh))))