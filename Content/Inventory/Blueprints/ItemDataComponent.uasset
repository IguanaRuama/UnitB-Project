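; Item data component that makes its owning actor a pickup carrying an item ID and quantity.
; On Interact, it looks up the instigator's BP_InventoryManager component and tries to add the item, destroying the owner when that succeeds.
; An instigator without that component only triggers an "Invalid" debug print, and Look At returns an empty string.
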(event EventInteract
  (params (Instigator :type Actor%20Object%20Reference))
  (bind _output_get (Variables|Default|SetInteract%20Instigator Instigator))
  (Utilities|IsValid (Actor|GetComponentbyClass _output_get "/Game/Inventory/Blueprints/BP_InventoryManager.BP_InventoryManager_C")
    (:Is%20Valid
      (bind _success (Default|AddtoInventory (Actor|GetComponentbyClass _output_get "/Game/Inventory/Blueprints/BP_InventoryManager.BP_InventoryManager_C") (.rowname (Variables|Default|GetItemID)) (Variables|Default|GetQuantity)))
      (if _success
        (Actor|DestroyActor (Components|GetOwner))))
    (:Is%20Not%20Valid
      (Development|PrintString "Invalid"))))

(fn Lookat
  (return ""))