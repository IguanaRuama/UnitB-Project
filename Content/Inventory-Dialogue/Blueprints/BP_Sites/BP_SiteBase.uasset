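; BP_SiteBase is a base site actor that shows a Widget component while the player's first-person character is inside its Box trigger.
; BeginPlay creates a WB_Weapon_Site widget and caches the player character for the overlap checks; this graph never adds that widget to the viewport.
; End overlap hides the component for the player, but restores game-only input, hides the cursor and removes the site widget for any actor.
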(event OnComponentBeginOverlap(Box)
  (params (OverlappedComponent :type Primitive%20Component%20Object%20Reference) (OtherActor :type Actor%20Object%20Reference) (OtherComp :type Primitive%20Component%20Object%20Reference) (OtherBodyIndex :type Integer) (bFromSweep :type Boolean) (SweepResult :type Hit%20Result%20Structure%20%28by%20ref%29))
  (if (== OtherActor (Variables|Default|GetAs%20BP%20First%20Person%20Character))
    (Rendering|SetVisibility (Variables|Default|GetWidget) true false)))

(event OnComponentEndOverlap(Box)
  (params (OverlappedComponent :type Primitive%20Component%20Object%20Reference) (OtherActor :type Actor%20Object%20Reference) (OtherComp :type Primitive%20Component%20Object%20Reference) (OtherBodyIndex :type Integer))
  (Utilities|FlowControl|Sequence
    (:then_0
      (if (== OtherActor (Variables|Default|GetAs%20BP%20First%20Person%20Character))
        (Rendering|SetVisibility (Variables|Default|GetWidget) false false)))
    (:then_1
      (Input|SetInputModeGameOnly (Game|GetPlayerController 0) false)
      (Variables|/Script/Engine.PlayerController|SetbShowMouseCursor (Game|GetPlayerController 0) false)
      (Widget|RemovefromParent (Variables|Default|GetSite%20Widget)))))

(event EventBeginPlay
  (bind _returnvalue (UserInterface|CreateWidget "/Game/Inventory-Dialogue/Widgets/WB_Sites/WB_Weapon_Site.WB_Weapon_Site_C"))
  (Variables|Default|SetSite%20Widget _returnvalue)
  (bind _asbp_first_person_character (Utilities|Casting|CastToBP_FirstPersonCharacter (Game|GetPlayerCharacter 0)))
  (Variables|Default|SetAs%20BP%20First%20Person%20Character _asbp_first_person_character))

(fn ConstructionScript)