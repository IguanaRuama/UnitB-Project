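; Weapon site Blueprint that opens and closes its site widget when interacted with, gated behind a first upgrade.
; The Interactor event stores the instigator and reads UpgradeFirstBool from the first WB_Upgrade widget found, printing a requirement message if it is false.
; When unlocked, it toggles SiteWidget in the viewport, switching input mode and mouse cursor to match.
; Its LookAt function returns an empty string.
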(event EventBeginPlay
  (|CallParentFunction) ; This node is disabled and will not be called.\nDrag off pins to build functionality.
)

(event EventInteractor
  (params (Instigator :type Actor%20Object%20Reference) (Player :type BP%20First%20Person%20Character%20Object%20Reference))
  (bind _returnvalue (Game|GetPlayerController 0))
  (bind _site_widget (Variables|Default|GetSite%20Widget))
  (Variables|Default|SetInteract%20Instigator Instigator)
  (bind _foundwidgets (Widget|GetAllWidgetsOfClass "/Game/Inventory-Dialogue/Widgets/WB_Old/WB_Upgrade.WB_Upgrade_C" false))
  (if (Variables|/Game/Inventory-Dialogue/Widgets/WB_Old/WB_Upgrade.WB_Upgrade_C|GetUpgrade_First_Bool (Utilities|Array|Get(acopy) _foundwidgets))
    (if (Widget|IsVisible (Variables|Default|GetSite%20Widget))
      (Input|SetInputModeGameOnly _returnvalue false)
      (Variables|/Script/Engine.PlayerController|SetbShowMouseCursor (Game|GetPlayerController 0) false)
      (Widget|RemovefromParent _site_widget)
      (else
        (Input|SetInputModeGameandUI _returnvalue _site_widget "DoNotLock" true false)
        (Variables|/Script/Engine.PlayerController|SetbShowMouseCursor (Game|GetPlayerController 0) true)
        (UserInterface|Viewport|AddtoViewport _site_widget 0)))
    (else
      (Development|PrintString "First Upgrade Required"))))

(fn ConstructionScript
  (|CallParentFunction))

(fn Lookat
  (return ""))