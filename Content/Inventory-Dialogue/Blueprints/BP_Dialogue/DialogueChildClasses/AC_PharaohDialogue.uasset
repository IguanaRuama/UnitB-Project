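; Dialogue child class for the Pharaoh, who demands the player's riches and reacts to the answer.
; It overrides the parent Dialouge function, calls it, then builds a two-choice branch with AddDialouge, switching on its returned state and option index.
; Agreeing earns thanks and refusing earns a curse, each followed by a Continue option that clears dialogue progress and closes the conversation.
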(fn Dialouge
  (|CallParentFunction)
  (bind (_state _option_index) (CallFunction|AddDialouge "Pharaoh" "Give me your riches!" (Utilities|Array|MakeArray "Fine" "No way!")))
  (switch Utilities|FlowControl|Switch|SwitchonEnum_Dialogue _state
    (:NewEnumerator0
      (switch int _option_index
        (:0
          (bind _state_2 (CallFunction|AddDialouge "Pharaoh" "You have my thanks, my loyal servant." (Utilities|Array|MakeArray "Continue")))
          (switch Utilities|FlowControl|Switch|SwitchonEnum_Dialogue _state_2
            (:NewEnumerator0
              (CallFunction|ClearDialogueProgress)
              (CallFunction|CloseConversation))))
        (:1
          (bind _state_3 (CallFunction|AddDialouge "Pharaoh" "Curse you! You will regret this!" (Utilities|Array|MakeArray "Continue")))
          (switch Utilities|FlowControl|Switch|SwitchonEnum_Dialogue _state_3
            (:NewEnumerator0
              (CallFunction|ClearDialogueProgress)
              (CallFunction|CloseConversation))))))))