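; Inventory manager that holds a fixed-size array of item slots and detects what the player camera is looking at.
; Adding items fills matching stacks one unit at a time up to the Item_Data stack size, then uses empty slots, returning any remainder.
; Each tick, a camera sphere trace tracks LookAtActor and prints its look-at message when the target changes.
; RemoveFromInventory is an empty stub; key 1 prints slot contents for debugging.
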(event EventBeginPlay
  (Utilities|Array|Resize (Variables|Default|GetContent) (Variables|Default|GetInventorySize)))

(event EventTick
  (params (DeltaSeconds :type Float%20%28single-precision%29))
  (CallFunction|Trace))

(event Input|KeyboardEvents|1
  (params (Key :type Key%20Structure :default "None"))
  (:Pressed
    (CallFunction|DEBUG)))

(fn AddtoInventory
  (params (ItemID :type Name) (Quantity :type Integer))
  (LocalVariables|SetQuantity%20Remaining Quantity)
  (while (and (> (LocalVariables|GetQuantity%20Remaining) 0) (not (LocalVariables|GetHasFailed)))
    (bind (_index _foundslot) (CallFunction|FindSlot ItemID))
    (if _foundslot
      (CallFunction|AddtoStack _index 1)
      (Math|Integer|DecrementInt (LocalVariables|GetQuantity%20Remaining))
      (elif (.IsEmptySlot (CallFunction|AnyEmptySlotsAvailable))
        (bind _success (CallFunction|CreateNewStack ItemID 1))
        (if _success
          (Math|Integer|DecrementInt (LocalVariables|GetQuantity%20Remaining))
          (else
            (LocalVariables|SetHasFailed true)))
        (else
          (LocalVariables|SetHasFailed true)))))
  (return (not (LocalVariables|GetHasFailed)) (LocalVariables|GetQuantity%20Remaining)))

(fn RemovefromInventory)

(fn FindSlot
  (params (ItemID :type Name))
  (for (_array_element _array_index) (Variables|Default|GetContent)
    (if (== (.ItemID (Utilities|Struct|BreakS_Slot _array_element)) ItemID)
      (if (< (.Quantity (Utilities|Struct|BreakS_Slot _array_element)) (CallFunction|GetMaxStackSize ItemID))
        (return _array_index true))))
  (return -1 false))

(fn GetMaxStackSize
  (params (ItemID :type Name))
  (bind _returnvalue (Utilities|GetDataTableRow "/Game/Inventory-Dialogue/Blueprints/BP_Inventory/Item_Data.Item_Data" ItemID)
    (:then
      (return (Utilities|Struct|BreakS_Item _returnvalue)))
    (:RowNotFound
      (return -1))))

(fn AddtoStack
  (params (Index :type Integer) (Quantity :type Integer))
  (bind _content (Variables|Default|GetContent))
  (bind _output (Utilities|Array|Get(acopy) _content Index))
  (Utilities|Array|SetArrayElem (Variables|Default|GetContent) Index (Utilities|Struct|MakeS_Slot (.itemid _output) (+ (.quantity _output) Quantity))))

(fn AnyEmptySlotsAvailable
  (for (_array_element _array_index) (Variables|Default|GetContent)
    (if (== (Utilities|Struct|BreakS_Slot _array_element) 0)
      (return true _array_index)))
  (return false -1))

(fn CreateNewStack
  (params (ItemID :type Name) (Quantity :type Integer))
  (bind (_isemptyslot _emptyindex) (CallFunction|AnyEmptySlotsAvailable))
  (if _isemptyslot
    (Utilities|Array|SetArrayElem (Variables|Default|GetContent) _emptyindex (Utilities|Struct|MakeS_Slot ItemID Quantity))
    (return true)
    (else
      (return false))))

(fn DEBUG
  (for (_array_element _array_index) (Variables|Default|GetContent)
    (Development|PrintString (Utilities|String|Append (Utilities|String|ToString(Integer) _array_index) ": " (Utilities|String|ToString(Name) (.ItemID (Utilities|Struct|BreakS_Slot _array_element))) " = " (Utilities|String|ToString(Integer) (.Quantity (Utilities|Struct|BreakS_Slot _array_element)))))))

(fn Trace
  (bind _returnvalue (Game|GetPlayerCameraManager 0))
  (bind _returnvalue_2 (Transformation|GetActorLocation _returnvalue))
  (bind (_outhit _returnvalue_3) (Collision|SphereTraceByChannel _returnvalue_2 (+ _returnvalue_2 (* (Transformation|GetActorForwardVector _returnvalue) (Variables|Default|GetTrace%20Range))) 15.0 "TraceTypeQuery3" false (Utilities|Array|MakeArray (Components|GetOwner)) "None"))
  (if _returnvalue_3
    (if (!= (.HitActor (Collision|BreakHitResult _outhit)) (Variables|Default|Get%20Look%20At%20Actor))
      (bind _output_get (Variables|Default|Set%20Look%20At%20Actor (.HitActor (Collision|BreakHitResult _outhit))))
      (bind _messasge (Class|BPIInterface|Lookat(Message) _output_get))
      (Development|PrintString (Utilities|String|ToString(Text) _messasge)))
    (else
      (Variables|Default|Set%20Look%20At%20Actor 0))))

(fn Lookat
  (return ""))