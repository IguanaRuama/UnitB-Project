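; Actor component that marks an item as pickable in the inventory system, holding its item ID and quantity.
; On interaction it stores the instigator and adds the item to the player's BPInventoryManager.
; A successful add destroys the owning actor, while a failed one prints a debug message.
; Its Look At function returns an empty string.
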(event EventInteractor
  (params (Instigator :type Actor%20Object%20Reference) (Player :type BP%20First%20Person%20Character%20Object%20Reference))
  (bind _bp_inventorymanager (Variables|/Game/FirstPerson/Blueprints/BP_FirstPersonCharacter.BP_FirstPersonCharacter_C|GetBP_InventoryManager Player))
  (Variables|Default|SetInteract%20Instigator Instigator)
  (Utilities|IsValid _bp_inventorymanager
    (:Is%20Valid
      (bind _success (Default|AddtoInventory _bp_inventorymanager (.rowname (Variables|Default|GetItemID)) (Variables|Default|GetQuantity)))
      (if _success
        (Actor|DestroyActor (Components|GetOwner))
        (else
          (Development|PrintString "Nope"))))))

(fn Lookat
  (return ""))