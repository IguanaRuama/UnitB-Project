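; BP_UserInterface handles key input for opening and closing the player menu and upgrade screens.
; BeginPlay creates one WB_PlayerMenu and one WB_Upgrade widget and keeps references to reuse.
; Tab toggles the menu and U toggles upgrades, adding or removing the widget from the viewport and switching input mode and mouse cursor to match.
; Each toggle checks only its own widget's visibility, independent of the other.
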(event EventBeginPlay
  (Utilities|FlowControl|Sequence
    (:then_0
      (bind _returnvalue (UserInterface|CreateWidget "/Game/Inventory-Dialogue/Widgets/WB_Inventory/WB_PlayerMenu.WB_PlayerMenu_C"))
      (Variables|Default|SetNewInvWidget _returnvalue))
    (:then_1
      (bind _returnvalue_2 (UserInterface|CreateWidget "/Game/Inventory-Dialogue/Widgets/WB_Old/WB_Upgrade.WB_Upgrade_C"))
      (Variables|Default|SetUpgradeWidget _returnvalue_2))))

(event Input|KeyboardEvents|Tab
  (params (Key :type Key%20Structure :default "None"))
  (bind _returnvalue (Game|GetPlayerController 0))
  (bind _newinvwidget (Variables|Default|GetNewInvWidget))
  (bind _newinvwidget_2 (Variables|Default|GetNewInvWidget))
  (:Pressed
    (if (Widget|IsVisible _newinvwidget)
      (Input|SetInputModeGameOnly _returnvalue false)
      (Variables|/Script/Engine.PlayerController|SetbShowMouseCursor (Game|GetPlayerController 0) false)
      (Widget|RemovefromParent _newinvwidget_2)
      (else
        (Input|SetInputModeGameandUI _returnvalue _newinvwidget "DoNotLock" true false)
        (Variables|/Script/Engine.PlayerController|SetbShowMouseCursor (Game|GetPlayerController 0) true)
        (UserInterface|Viewport|AddtoViewport _newinvwidget_2 0)))))

(event Input|KeyboardEvents|U
  (params (Key :type Key%20Structure :default "None"))
  (bind _returnvalue (Game|GetPlayerController 0))
  (bind _upgradewidget (Variables|Default|GetUpgradeWidget))
  (bind _upgradewidget_2 (Variables|Default|GetUpgradeWidget))
  (:Pressed
    (if (Widget|IsVisible _upgradewidget_2)
      (Input|SetInputModeGameOnly _returnvalue false)
      (Variables|/Script/Engine.PlayerController|SetbShowMouseCursor (Game|GetPlayerController 0) false)
      (Widget|RemovefromParent _upgradewidget)
      (else
        (Input|SetInputModeGameandUI _returnvalue _upgradewidget_2 "DoNotLock" true false)
        (Variables|/Script/Engine.PlayerController|SetbShowMouseCursor (Game|GetPlayerController 0) true)
        (UserInterface|Viewport|AddtoViewport _upgradewidget 0)))))