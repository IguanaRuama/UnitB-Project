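; Base dialogue component that runs branching conversations through WB_Dialogue, switching mouse cursor and input mode on open and close.
; The empty Dialogue function, apparently meant for child overrides, is replayed from the start on every progress update.
; Each AddDialogue call returns the option stored in the DialogueProgress map for its index, or displays that line if none exists.
; Helpers record choices, roll back steps, or switch tree index and clear progress.
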(fn OpenConversation
  (bind _returnvalue (UserInterface|CreateWidget "/Game/Dialogue/Widgets/WB_Dialogue.WB_Dialogue_C" (Game|GetPlayerController 0) self))
  (bind _output_get (Variables|Default|SetDialogue%20Widget _returnvalue))
  (UserInterface|Viewport|AddtoViewport _output_get 0)
  (CallFunction|ProgressDialogue)
  (Input|SetInputModeUIOnly (Game|GetPlayerController 0) 0 "DoNotLock" true)
  (Variables|/Script/Engine.PlayerController|SetbShowMouseCursor (Game|GetPlayerController 0) true))

(fn CloseConversation
  (bind _foundwidgets (Widget|GetAllWidgetsOfClass "/Game/Dialogue/Widgets/WB_Dialogue.WB_Dialogue_C" true))
  (for _array_element _foundwidgets
    (Widget|RemovefromParent _array_element)
    (Variables|/Script/Engine.PlayerController|SetbShowMouseCursor (Game|GetPlayerController 0) false)
    (Input|SetInputModeGameOnly (Game|GetPlayerController 0) false)))

(fn ProgressDialogue
  (Variables|Default|SetDialogue%20Index -1)
  (CallFunction|Dialogue))

(fn Dialogue)

(fn AddDialogue
  (params (Speaker :type Text) (Dialogue :type Text) (Dialogue%20Options :type Array%20of%20Texts))
  (bind _dialogue_progress (Variables|Default|GetDialogue%20Progress))
  (bind _dialogue_index (Variables|Default|GetDialogue%20Index))
  (bind (_value _returnvalue) (Utilities|Map|Find _dialogue_progress _dialogue_index))
  (Math|Integer|IncrementInt (Variables|Default|GetDialogue%20Index)
    (:%20%20
      (if _returnvalue
        (return "NewEnumerator0" _value)
        (else
          (Default|UpdateDialogueText (Variables|Default|GetDialogue%20Widget) (Variables|Default|GetDialogue%20Index) Speaker Dialogue Dialogue%20Options)
          (return "NewEnumerator1" 0))))))

(fn UpdateSelectedProgress
  (params (Progress%20Index :type Integer%20%28by%20ref%29) (Option%20index :type Integer%20%28by%20ref%29))
  (Utilities|Map|Add (Variables|Default|GetDialogue%20Progress) Progress%20Index Option%20index)
  (CallFunction|ProgressDialogue))

(fn ClearDialogieProgress
  (Utilities|Map|Clear (Variables|Default|GetDialogue%20Progress)))

(fn RemoveDialogueProgress
  (params (Progress%20Steps :type Integer))
  (for _index (range 0 Progress%20Steps)
    (Utilities|Map|Remove (Variables|Default|GetDialogue%20Progress) (- (Variables|Default|GetDialogue%20Index) _index))))

(fn SetDialogueTreeIndex
  (params (Dialogue%20Tree%20Index :type Integer))
  (Variables|Default|SetDialogue%20Tree%20Index Dialogue%20Tree%20Index)
  (CallFunction|ClearDialogieProgress))