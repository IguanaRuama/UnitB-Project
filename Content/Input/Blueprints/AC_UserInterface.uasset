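; AC_UserInterface is a component that manages the player's inventory screen.
; On BeginPlay it creates and caches a WB_PlayerInventory widget.
; The IA_Inventory input action toggles that widget in the viewport, switching between Game Only and Game And UI input modes and hiding or showing the mouse cursor to match.
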(event Input|EnhancedActionEvents|EnhancedInputActionIA_Inventory
  (params (ActionValue :type Boolean) (ElapsedSeconds :type Float%20%28double-precision%29) (TriggeredSeconds :type Float%20%28double-precision%29) (InputAction :type Input%20Action%20Object%20Reference :default "/Game/Input/Actions/IA_Inventory.IA_Inventory"))
  (bind _returnvalue (Game|GetPlayerController 0))
  (bind _returnvalue_2 (Game|GetPlayerController 0))
  (bind _player_inventory (Variables|Default|GetPlayer%20Inventory))
  (:Started
    (if (Widget|IsVisible (Variables|Default|GetPlayer%20Inventory))
      (Widget|RemovefromParent _player_inventory)
      (Input|SetInputModeGameOnly _returnvalue false)
      (Variables|/Script/Engine.PlayerController|SetbShowMouseCursor _returnvalue_2 false)
      (else
        (UserInterface|Viewport|AddtoViewport _player_inventory 0)
        (Input|SetInputModeGameandUI _returnvalue _player_inventory "DoNotLock" false false)
        (Variables|/Script/Engine.PlayerController|SetbShowMouseCursor _returnvalue_2 true)))))

(event EventBeginPlay
  (bind _returnvalue (UserInterface|CreateWidget "/Game/Inventory/Widgets/WB_PlayerInventory.WB_PlayerInventory_C"))
  (Variables|Default|SetPlayer%20Inventory _returnvalue))